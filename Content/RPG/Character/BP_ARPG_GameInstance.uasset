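; RPG game instance that holds the selected save character, a cached settings widget and the latest network and travel errors.
; Network and travel failures print their type and store a red, timed message widget.
; ShowLastError later adds one to the viewport, preferring the network error, then clears both.
; GetSettingsWidget creates and returns the widget when none is valid; otherwise it only makes it visible.
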(event Custom|ShowLastError
  ;[1 1 1] Show last network errors
  (Utilities|IsValid (Variables|Default|GetLastNetworkError)
    (:Is%20Valid
      (UserInterface|Viewport|AddtoViewport (Variables|Default|GetLastNetworkError) 4))
    (:Is%20Not%20Valid
      (Utilities|IsValid (Variables|Default|GetLastTravelError)
        (:Is%20Valid
          (UserInterface|Viewport|AddtoViewport (Variables|Default|GetLastTravelError) 4)))))
  (Variables|Default|SetLastNetworkError 0)
  (Variables|Default|SetLastTravelError 0))

(event EventHandleNetworkError
  (params (FailureType :type ENetworkFailure%20Enum :default "NetDriverAlreadyExists") (bIsServer :type Boolean))
  (bind _returnvalue (Utilities|String|EnumtoString FailureType))
  (bind _result (Utilities|Text|FormatText "Networkd error Type: {Type}" _returnvalue))
  ;[1 1 1] Show last network errors
  (Development|PrintText _result)
  (bind _returnvalue_2 (UserInterface|CreateWidget "/Game/RPG/InventorySystem/JigSaw/Widgets/ContextMenu/BP_MessageWidget.BP_MessageWidget_C" 0 _result 5.0 "(R=1.000000,G=0.000000,B=0.000000,A=1.000000)"))
  (Variables|Default|SetLastNetworkError _returnvalue_2))

(event EventHandleTravelError
  (params (FailureType :type ETravelFailure%20Enum :default "NoLevel"))
  (bind _returnvalue (Utilities|String|EnumtoString FailureType))
  (bind _result (Utilities|Text|FormatText "Travel Error Type: {Type}" _returnvalue))
  ;[1 1 1] Show last network errors
  (Development|PrintText _result)
  (bind _returnvalue_2 (UserInterface|CreateWidget "/Game/RPG/InventorySystem/JigSaw/Widgets/ContextMenu/BP_MessageWidget.BP_MessageWidget_C" 0 _result 5.0 "(R=1.000000,G=0.000000,B=0.000000,A=1.000000)"))
  (Variables|Default|SetLastTravelError _returnvalue_2))

(fn SetSelectedCharacter
  (params (SelectedSaveCharacter :type S%20Saved%20Local%20Character%20Structure))
  (Variables|Default|SetSelectedSaveCharacter SelectedSaveCharacter)
  (Variables|Default|SetCharacterSelected? true))

(fn ClearSelectedCharacter
  (Variables|Default|SetSelectedSaveCharacter "")
  (Variables|Default|SetCharacterSelected? false))

(fn GetSelectedCharacter
  (return (Variables|Default|GetSelectedSaveCharacter) (Variables|Default|GetCharacterSelected?)))

(fn GetSettingsWidget
  (Utilities|IsValid (Variables|Default|GetSettingsWidget)
    (:Is%20Valid
      (Widget|SetVisibility (Variables|Default|GetSettingsWidget) "Visible"))
    (:Is%20Not%20Valid
      (bind _returnvalue (UserInterface|CreateWidget "/Game/RPG/Widgets/OtherWidgets/Settings/BP_SettingsWidget.BP_SettingsWidget_C"))
      (Variables|Default|SetSettingsWidget _returnvalue)
      (return (Variables|Default|GetSettingsWidget)))))