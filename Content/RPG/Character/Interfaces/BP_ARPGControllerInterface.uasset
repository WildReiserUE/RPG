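; Blueprint interface for the RPG player controller, declaring the calls other game systems make on it without casting to a concrete class.
; It exposes getters for the pawn, inventory and skill tree, plus notifications for item, equipment, mod and credit changes.
; Further functions cover death, skill targeting and movement abilities, input mode, chat, party membership and leadership, guild name and player interaction.
; All functions are stubs without logic.
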(fn GetControlledPawnRef
  (return 0))

(fn GetInventoryComponent
  (return 0))

(fn OnActionItemPickedUp
  (params (JigRef :type BP%20Jig%20Slot%20Object%20Reference))
  (return false))

(fn OnModRemoved
  (params (Info :type Container%20Items%20Structure))
  (return false))

(fn OnItemDropped
  (params (Info :type F%20Item%20Info%20Structure) (FromSlot :type EquipmentSlots%20Enum :default "NewEnumerator12"))
  (return false))

(fn OnItemConsumed
  (params (Info :type F%20Item%20Info%20Structure))
  (return false))

(fn OnModInstalled
  (params (Info :type Container%20Items%20Structure))
  (return false))

(fn OnItemEquipped
  (params (ToSlot :type EquipmentSlots%20Enum :default "NewEnumerator12") (ItemInfo :type F%20Item%20Info%20Structure) (CItems :type Array%20of%20Container%20Items%20Structures))
  (return false))

(fn OnPrimarySecondarySwapped
  (params (PrimaryInfo :type F%20Item%20Info%20Structure) (SecondaryInfo :type F%20Item%20Info%20Structure) (PrimaryEquipped? :type Boolean) (SecondaryEquipped :type Boolean))
  (return false))

(fn OnEquipementReplaced
  (params (Slot :type EquipmentSlots%20Enum :default "NewEnumerator12") (OldInfo :type F%20Item%20Info%20Structure) (NewItemInfo :type F%20Item%20Info%20Structure))
  (return false))

(fn OnItemBought
  (params (Info :type F%20Item%20Info%20Structure) (NewCredits :type Character%20Currency%20Structure))
  (return false))

(fn OnCreditsUpdated
  (params (NewCredits :type Character%20Currency%20Structure))
  (return false))

(fn OnItemSold
  (params (Info :type F%20Item%20Info%20Structure) (NewCredits :type Character%20Currency%20Structure))
  (return false))

(fn OnRingsSwapped
  (params (PrimaryInfo :type F%20Item%20Info%20Structure) (SecondaryInfo :type F%20Item%20Info%20Structure) (PrimaryEquipped? :type Boolean) (SecondaryEquipped :type Boolean))
  (return false))

(fn OnEarringSwapped
  (params (PrimaryInfo :type F%20Item%20Info%20Structure) (SecondaryInfo :type F%20Item%20Info%20Structure) (PrimaryEquipped? :type Boolean) (SecondaryEquipped :type Boolean))
  (return false))

(fn OnItemUnEquipped
  (params (ToSlot :type EquipmentSlots%20Enum :default "NewEnumerator12") (ItemInfo :type F%20Item%20Info%20Structure) (CItems :type Array%20of%20Container%20Items%20Structures))
  (return false))

(fn AddNewSubscriber
  (params (Player :type Player%20Controller%20Object%20Reference))
  (return false))

(fn ControlleronPlayerDeath
  (return false))

(fn ControllerMovetoSkillTarget
  (params (Target :type Actor%20Object%20Reference) (Range :type Float%20%28single-precision%29) (Actionbar :type E_ActionbarSlots%20Enum :default "NewEnumerator4"))
  (return false))

(fn GetSkillTreeComponent
  (return 0))

(fn ControllerHandleInputMode
  (return))

(fn ControllerSetLocalCharacter
  (params (LocalCharRef :type BP%20ARPG%20Local%20Character%20Object%20Reference))
  (return false))

(fn ControlleronSkillPerformed
  (return false))

(fn ControllerSendChatMessage
  (params (Message :type String) (MessageType :type E_ChatSectionType%20Enum :default "NewEnumerator0"))
  (return false))

(fn ControllerAddNewChatMessage
  (params (Message :type String) (FromPlayer :type String) (MessageType :type E_ChatSectionType%20Enum :default "NewEnumerator0"))
  (return false))

(fn ControllerHasParty
  (return false 0))

(fn ControllerAddPartyMember
  (params (NewMembers :type Pawn%20Object%20Reference))
  (return false))

(fn ControllerLeaveParty
  (return false))

(fn ControllerRemovePartyMember
  (params (NewMembers :type Pawn%20Object%20Reference))
  (return false))

(fn ControllerGetPartyLeader
  (return false 0))

(fn ControllerSetIsPartyLeader
  (params (IsPartyLeader :type Boolean))
  (return false))

(fn ControllerIsPartyLeader
  (return false))

(fn ControllerGetPartyMembers
  (return false 0))

(fn ControllerSetPartyMembers
  (params (Members :type Array%20of%20Pawn%20Object%20References))
  (return false))

(fn ControllerGetGuildName
  (return "None" false))

(fn ControllerGetMode
  (return "NewEnumerator0"))

(fn ControlleronAbilityTeleport
  (params (Location :type Vector) (Rotation :type Rotator))
  (return false))

(fn ControlleronAbilityLaunchCharacter
  (params (Rotation :type Rotator) (Velocity :type Vector) (XYOverride :type Boolean) (ZOverride :type Boolean))
  (return false))

(fn ControlleronInteractedwithPlayer
  (params (Player :type Actor%20Object%20Reference))
  (return false))