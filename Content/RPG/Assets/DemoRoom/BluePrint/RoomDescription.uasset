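; RoomDescription is a demo room Blueprint with a base mesh and a flat wall mesh that share a configurable stand color.
; Its construction script creates dynamic material instances on both meshes and sets their Color parameter from StandColor.
; BeginPlay, outside dedicated servers, checks the first player controller for a BP_InventoryComponent but takes no action on the result.
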(event EventBeginPlay
  (if (not (Networking|IsDedicatedServer))
    (Utilities|IsValid (Actor|GetComponentbyClass (Game|GetPlayerController 0) "/Game/RPG/Blueprints/Components/BP_InventoryComponent.BP_InventoryComponent_C"))))

(fn ConstructionScript
  (bind _returnvalue (Rendering|Material|CreateDynamicMaterialInstance (Variables|Default|GetSM_Base) 3 0 "None" :!class /Script/Engine.PrimitiveComponent))
  (Rendering|Material|SetVectorParameterValue _returnvalue "Color" (Variables|Default|GetStandColor) :!class /Script/Engine.MaterialInstanceDynamic)
  (bind _returnvalue_2 (Rendering|Material|CreateDynamicMaterialInstance (Variables|Default|GetSM_Base_FlatWall) 0 0 "None" :!class /Script/Engine.PrimitiveComponent))
  (Rendering|Material|SetVectorParameterValue _returnvalue_2 "Color" (Variables|Default|GetStandColor) :!class /Script/Engine.MaterialInstanceDynamic))