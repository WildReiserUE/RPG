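; BP_Outline is a post-process actor that draws a colored outline, apparently around objects marked in the custom depth buffer.
; On BeginPlay it creates a dynamic instance of the custom-depth outline material, sets a default golden color and installs it as a weighted blendable in its PostProcess settings.
; A ChangeColor event updates the Color parameter on that stored instance so the outline can be recolored at runtime.
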(event Custom|ChangeColor
  (params (Value :type Linear%20Color%20Structure))
  (Rendering|Material|SetVectorParameterValue (Variables|Default|GetDynmMat) "Color" Value :!class /Script/Engine.MaterialInstanceDynamic))

(event EventBeginPlay
  (bind _returnvalue (Rendering|Material|CreateDynamicMaterialInstance "/Game/RPG/Materials/Outline/M_OutlineCustomDepth_Inst.M_OutlineCustomDepth_Inst" "None" "None" :!class /Script/Engine.KismetMaterialLibrary))
  (bind _output_get (Variables|Default|SetDynmMat _returnvalue))
  (Rendering|Material|SetVectorParameterValue _output_get "Color" "(R=1.000000,G=0.744141,B=0.000000,A=1.000000)" :!class /Script/Engine.MaterialInstanceDynamic)
  (Variables|/Script/Engine.PostProcessComponent|SetSettings (Variables|Default|GetPostProcess) (Utilities|Struct|MakePostProcessSettings (Utilities|Struct|MakeWeightedBlendables (Utilities|Array|MakeArray (Utilities|Struct|MakeWeightedBlendable 1.0 _returnvalue))))))

(fn ConstructionScript)