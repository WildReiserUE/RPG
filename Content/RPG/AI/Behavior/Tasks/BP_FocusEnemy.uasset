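; Behavior tree task that turns an AI character to face its current enemy in combat.
; It disables orient-rotation-to-movement on the BP_AI_Main pawn, stops the controller's movement and sets focus on the Enemy blackboard actor.
; After a configurable delay, it finishes successfully, leaving the focus and rotation setting in place.
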(event EventReceiveExecuteAI
  (params (OwnerController :type AI%20Controller%20Object%20Reference) (ControlledPawn :type Pawn%20Object%20Reference))
  (Utilities|FlowControl|Sequence
    (:then_0
      (bind _asbp_ai_main (Utilities|Casting|CastToBP_AI_Main ControlledPawn))
      (Variables|/Script/Engine.CharacterMovementComponent|SetbOrientRotationToMovement (Variables|/Script/Engine.Character|GetCharacterMovement _asbp_ai_main) false))
    (:then_1
      (AI|Navigation|StopMovement OwnerController)
      (AI|SetFocus OwnerController (AI|BehaviorTree|GetBlackboardValueasActor (Variables|Default|GetEnemy)))
      (Utilities|FlowControl|Delay (Variables|Default|GetDelay))
      (AI|BehaviorTree|FinishExecute true))))