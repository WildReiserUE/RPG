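; Behavior tree task that has a guard AI face and strafe around its blackboard enemy within strafe range, failing when it can attack or is out of range.
; FindStrafingLocation tries navmesh points: backstep when too close, random angled side, opposite side, then farther back, otherwise moving toward the enemy.
; Tick records the enemy's last known location and aborts on range loss, target change, stun or, if defensive, safe-zone exit.
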(event Custom|ProcessMove
  (bind _distance (Variables|Default|GetDistance))
  (if (> _distance (* (Variables|Default|GetDistanceFromTargetToStrafeVal) 1.5))
    (Variables|Default|SetMovingToTarget true :!label _label)
    (Default|SetWalkRun (Variables|Default|GetAIPawn) (> _distance (* (Variables|Default|GetDistanceFromTargetToStrafeVal) 2.0)) false)
    (AI|AIMoveTo (Variables|Default|GetController) "0, 0, 0" (Variables|Default|GetEnemyRef) (Class|BTFunctionLibrary|GetBlackboardValueasFloat (Variables|Default|GetRaduis)) "Default" "Default" true false
      (:OnRequestFailed
        (AI|BehaviorTree|FinishExecute false))
      (:OnMoveFinished
        (AI|BehaviorTree|FinishExecute true)))
    (else
      (Variables|Default|SetMovingToTarget false)
      (bind (_result _location) (CallFunction|FindStrafingLocation))
      (if _result
        (Default|SetWalkRun (Variables|Default|GetAIPawn) false true)
        (AI|AIMoveTo (Variables|Default|GetController) _location 0 3e+01 "Default" "Default" true false
          (:OnRequestFailed
            (AI|BehaviorTree|FinishExecute false))
          (:OnMoveFinished
            (AI|BehaviorTree|FinishExecute true)))
        (else
          (goto _label))))))

(event EventReceiveExecuteAI
  (params (OwnerController :type AI%20Controller%20Object%20Reference) (ControlledPawn :type Pawn%20Object%20Reference))
  (Variables|Default|SetStrafeDistanceValue (Class|BTFunctionLibrary|GetBlackboardValueasFloat (Variables|Default|GetStrafeDistance)))
  (bind _output_get (Variables|Default|SetDistanceFromTargetToStrafeVal (Class|BTFunctionLibrary|GetBlackboardValueasFloat (Variables|Default|GetDistanceFromActorToStrafe))))
  (if (> _output_get 0.0)
    (Variables|Default|SetStrafeAngleValue (Class|BTFunctionLibrary|GetBlackboardValueasFloat (Variables|Default|GetStrafeAngle)))
    (Variables|Default|SetController OwnerController)
    (bind _output_get_2 (Variables|Default|SetEnemyRef (AI|BehaviorTree|GetBlackboardValueasActor (Variables|Default|GetEnemy))))
    (Utilities|IsValid _output_get_2
      (:Is%20Valid
        (bind _asbp_ai_main (Utilities|Casting|CastToBP_AI_Main ControlledPawn))
        (bind _output_get_3 (Variables|Default|SetAIPawn _asbp_ai_main))
        (bind _output_get_4 (Variables|Default|SetDistance (Math|Vector|VectorLength (- (Transformation|GetActorLocation _output_get_3) (Transformation|GetActorLocation _output_get_2)))))
        (if (and (Default|HasValidAttackIndex _output_get_3) (Default|CanAttack _output_get_3))
          (Default|SetWalkRun _output_get_3 (not (> _output_get_4 (* (Variables|Default|GetDistanceFromTargetToStrafeVal) 1.1))) false)
          (AI|BehaviorTree|FinishExecute false :!label _label)
          (elif (> _output_get_4 (* (Variables|Default|GetDistanceFromTargetToStrafeVal) 1.1))
            (Default|SetWalkRun (Variables|Default|GetAIPawn) false false)
            (goto _label)
            (else
              (AI|SetFocus (Variables|Default|GetController) (Variables|Default|GetEnemyRef))
              (Variables|/Script/Engine.CharacterMovementComponent|SetbOrientRotationToMovement (Variables|/Script/Engine.Character|GetCharacterMovement (Variables|Default|GetAIPawn)) false)
              (Default|SetWalkRun (Variables|Default|GetAIPawn) true false)
              (if (> (Variables|Default|GetDistance) (* (Variables|Default|GetDistanceFromTargetToStrafeVal) 1.5))
                (Variables|Default|SetMovingToTarget true :!label _label_2)
                (Default|SetWalkRun (Variables|Default|GetAIPawn) (> (Variables|Default|GetDistance) (* (Variables|Default|GetDistanceFromTargetToStrafeVal) 2.0)) false)
                (AI|AIMoveTo (Variables|Default|GetController) "0, 0, 0" (Variables|Default|GetEnemyRef) (Class|BTFunctionLibrary|GetBlackboardValueasFloat (Variables|Default|GetRaduis)) "Default" "Default" true false
                  (:OnRequestFailed
                    (AI|BehaviorTree|FinishExecute false))
                  (:OnMoveFinished
                    (AI|BehaviorTree|FinishExecute true)))
                (else
                  (Variables|Default|SetMovingToTarget false)
                  (bind (_result _location) (CallFunction|FindStrafingLocation))
                  (if _result
                    (Default|SetWalkRun (Variables|Default|GetAIPawn) false true)
                    (AI|AIMoveTo (Variables|Default|GetController) _location 0 3e+01 "Default" "Default" true false
                      (:OnRequestFailed
                        (AI|BehaviorTree|FinishExecute false))
                      (:OnMoveFinished
                        (AI|BehaviorTree|FinishExecute true)))
                    (else
                      (goto _label_2))))))))))
    (else
      (AI|BehaviorTree|FinishExecute false))))

(event EventTick
  (params (OwnerActor :type Actor%20Object%20Reference) (DeltaSeconds :type Float%20%28single-precision%29))
  (bind _enemyref (Variables|Default|GetEnemyRef))
  (Utilities|IsValid _enemyref
    (:Is%20Valid
      (AI|BehaviorTree|SetBlackboardValueasVector (Variables|Default|GetLastKnownLoc) (Transformation|GetActorLocation _enemyref))
      (bind _output_get (Variables|Default|SetDistance (Math|Vector|VectorLength (- (Transformation|GetActorLocation (Variables|Default|GetAIPawn)) (Transformation|GetActorLocation _enemyref)))))
      (if (> _output_get (* (Variables|Default|GetDistanceFromTargetToStrafeVal) 1.1))
        (Default|SetWalkRun (Variables|Default|GetAIPawn) true false)
        (AI|BehaviorTree|FinishExecute false :!label _label)
        (else
          (if (Variables|Default|GetIsDefensive)
            (if (not (Default|IsTargetWithinSafeZone (Variables|Default|GetAIPawn) (Variables|Default|GetEnemyRef)))
              (Default|SetWalkRun (Variables|Default|GetAIPawn) false false)
              (goto _label)
              (else
                _)))
          (Utilities|FlowControl|Sequence
            (:then_0
              (if (Variables|Default|GetMovingToTarget)
                (if (not (> (Variables|Default|GetDistance) (* (Variables|Default|GetDistanceFromTargetToStrafeVal) 1.1)))
                  (AI|Navigation|StopMovement (Variables|Default|GetController))
                  (CallFunction|ProcessMove))
                (elif (> (Variables|Default|GetDistance) (* (Variables|Default|GetDistanceFromTargetToStrafeVal) 1.1))
                  (AI|Navigation|StopMovement (Variables|Default|GetController))
                  (CallFunction|ProcessMove))))
            (:then_1
              (bind _output_get_2 (Default|SetNewTarget (Variables|Default|GetAIPawn)))
              (if (or (!= _output_get_2 (Variables|Default|GetEnemyRef)) (Default|IsStunned? (Variables|Default|GetAIPawn)))
                (Default|SetWalkRun (Variables|Default|GetAIPawn) true false)
                (AI|Navigation|StopMovement (Variables|Default|GetController))
                (AI|BehaviorTree|FinishExecute false)))))))))

(fn FindStrafingLocation
  (bind _aipawn (Variables|Default|GetAIPawn))
  (bind _aipawn_2 (Variables|Default|GetAIPawn))
  (bind _aipawn_3 (Variables|Default|GetAIPawn))
  (if (and (< (Variables|Default|GetDistance) (+ (Class|BTFunctionLibrary|GetBlackboardValueasFloat (Variables|Default|GetRaduis)) 2e+01)) (not (and (Default|HasValidAttackIndex _aipawn_3) (Default|CanAttack _aipawn_3))))
    (bind _output_get (LocalVariables|SetLoc (+ (Transformation|GetActorLocation _aipawn) (* (Transformation|GetActorForwardVector _aipawn) -5e+01))))
    (bind (_randomlocation _returnvalue) (Class|NavigationSystemV1|GetRandomLocationinNavigableRadius _output_get 1e+02 0 0))
    (Variables|Default|SetResultLoc _randomlocation)
    (if _returnvalue
      _
      (else
        (bind _output_get_2 (Variables|Default|SetRandBool (Math|Random|RandomBool) :!label _label))
        (bind _output_get_3 (LocalVariables|SetLoc (CallFunction|GetStrafeLoc _output_get_2)))
        (bind (_randomlocation_2 _returnvalue_2) (Class|NavigationSystemV1|GetRandomLocationinNavigableRadius _output_get_3 3e+01 0 0))
        (Variables|Default|SetResultLoc _randomlocation_2)
        (if _returnvalue_2
          _
          (else
            (bind _output_get_4 (LocalVariables|SetLoc (CallFunction|GetStrafeLoc (not (Variables|Default|GetRandBool)))))
            (bind (_randomlocation_3 _returnvalue_3) (Class|NavigationSystemV1|GetRandomLocationinNavigableRadius _output_get_4 3e+01 0 0))
            (if _returnvalue_3
              (Variables|Default|SetResultLoc _randomlocation_3)
              (else
                (bind _output_get_5 (LocalVariables|SetLoc (+ (Transformation|GetActorLocation _aipawn_2) (* (Transformation|GetActorForwardVector _aipawn_2) -1e+02))))
                (bind (_randomlocation_4 _returnvalue_4) (Class|NavigationSystemV1|GetRandomLocationinNavigableRadius _output_get_5 1e+02 0 0))
                (if _returnvalue_4
                  (Variables|Default|SetResultLoc _randomlocation_4)
                  (else
                    (return false "0, 0, 0")))))))))
    (else
      (goto _label)))
  (return true (Variables|Default|GetResultLoc)))

(fn GetStrafeLoc
  (params (RandBool :type Boolean))
  (bind _strafeanglevalue (Variables|Default|GetStrafeAngleValue))
  (bind _aipawn (Variables|Default|GetAIPawn))
  (return (+ (Transformation|GetActorLocation _aipawn) (* (Math|Vector|RotateVector (Transformation|GetActorRightVector _aipawn) (Math|Rotator|SelectRotator (Math|Rotator|MakeRotator 0.0 0.0 (* _strafeanglevalue -1.0)) (Math|Rotator|MakeRotator 0.0 0.0 (+ _strafeanglevalue 1.8e+02)) RandBool)) (Variables|Default|GetStrafeDistanceValue)))))