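; AI preset for an NPC that stays non-hostile until damaged, then turns its whole party against the damage causer.
; On damage, a hostility check gates activating each party member, switching its behavior, adding aggro and either targeting or investigating undetected damage.
; On the server, losing the target starts a retriggerable ten-second delay that restores passive behavior and clears aggro if still targetless.
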(event Custom|OnNewTargetSet_Event_0
  (params (Enemy :type Actor%20Object%20Reference))
  ;[1 1 1] Becomes non hostile once they have no target for 10 seconds.
  (Utilities|IsValid Enemy
    (:Is%20Not%20Valid
      (Utilities|FlowControl|RetriggerableDelay 1e+01)
      (if (not (.ReturnValue (CallFunction|HasEnemyTarget)))
        (CallFunction|SetHostility "NewEnumerator5")
        (CallFunction|ClearAggroTargets)
        (Variables|Default|SetAIBehaviorType "NewEnumerator3")))))

(event Custom|MC_SetAggroIndicator
  (params (IsAggro :type Boolean))
  ;[1 1 1] MC aggro state
  (CallFunction|SetPlayerHostilityDanger IsAggro))

(event Game|Damage|EventAnyDamage
  (params (Damage :type Float%20%28single-precision%29) (DamageType :type Damage%20Type%20Object%20Reference) (InstigatedBy :type Controller%20Object%20Reference) (DamageCauser :type Actor%20Object%20Reference))
  ;[1 1 1] This AI will not attack the player unless damaged by the player
  (|CallParentFunction Damage DamageType InstigatedBy DamageCauser)
  (Utilities|IsValid DamageCauser
    (:Is%20Valid
      (bind _result (Class|ITInteractInterface|GetAIHostility(Message) DamageCauser))
      (if (Utilities|Enum|NotEqual(Enum) _result "NewEnumerator3")
        (bind _output_get (CallFunction|GetAllPartyMembers))
        (for _array_element _output_get
          (Utilities|IsValid _array_element
            (:Is%20Valid
              (if (not (Default|CheckActorAggro _array_element DamageCauser))
                (Utilities|FlowControl|Sequence
                  (:then_0
                    (if (not (Variables|/Game/RPG/AI/BP_AI_Main.BP_AI_Main_C|GetIsAIActive _array_element))
                      (Default|ActivateAI _array_element)))
                  (:then_1
                    (if (Utilities|Enum|Equal(Enum) (Variables|/Game/RPG/AI/BP_AI_Main.BP_AI_Main_C|GetAIBehaviorType _array_element) "NewEnumerator3")
                      (Variables|/Game/RPG/AI/BP_AI_Main.BP_AI_Main_C|SetAIBehaviorType _array_element "NewEnumerator0")))
                  (:then_2
                    (Default|AddAggroTarget _array_element DamageCauser)
                    (if (not (.ReturnValue (Default|HasEnemyTarget _array_element)))
                      (if (Variables|Default|GetInvestigateUndetectedDamage?)
                        (Default|CheckTakenDamagefromFog _array_element DamageCauser)
                        (else
                          (Default|SetNewTarget _array_element))))))))))))))

(event EventBeginPlay
  ;[1 1 1] Becomes non hostile once they have no target for 10 seconds.
  (|CallParentFunction)
  (Networking|SwitchHasAuthority
    (:Authority
      (EventDispatchers|AssignOnNewTargetSet (delegate Custom|OnNewTargetSet_Event_0)))))

(fn ConstructionScript
  (|CallParentFunction)
  (Class|SkinnedMeshComponent|SetMasterPoseComponent (Variables|Default|GetArmor_0) (Variables|Character|GetMesh) false))

(fn GetAllPartyMembers
  (bind _output_get (LocalVariables|SetMem (CallFunction|GetAIParty)))
  (Utilities|Array|AddUnique _output_get self) ; In case Mem length = 0
  (return (LocalVariables|GetMem)))