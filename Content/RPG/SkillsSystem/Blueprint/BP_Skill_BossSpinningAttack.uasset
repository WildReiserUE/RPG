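; Boss spinning attack skill actor that deals area damage around its owning pawn as soon as it spawns.
; On the server, BeginPlay runs a multi-sphere object trace centred just above the owner, ignoring the owner, and damages the hits using the skill's damage and damage type.
; It then applies skill effects to each returned enemy and destroys itself, making it a one-shot instant hit.
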(event EventBeginPlay
  (bind _pawnowner (Variables|Default|GetPawnOwner))
  (bind _returnvalue (Transformation|GetActorLocation _pawnowner))
  (bind _returnvalue_2 (+ _returnvalue "0, 0,30.000000"))
  ;[1 1 1] Deals aoe damage using a sphere trace
  (|CallParentFunction)
  (Utilities|FlowControl|Sequence
    (:then_0
      (Networking|SwitchHasAuthority
        (:Authority
          (bind _outhits (Collision|MultiSphereTraceForObjects _returnvalue_2 _returnvalue_2 2e+02 (Utilities|Array|MakeArray "ObjectTypeQuery3" "ObjectTypeQuery2") false (Utilities|Array|MakeArray (Variables|Default|GetPawnOwner)) "None"))
          (bind _hitenemies (CallFunction|DamageMultipleEnemies _outhits (Variables|Default|GetSkillDamage) (Variables|Default|GetDamageType)))
          (for _array_element _hitenemies
            (CallFunction|ApplySkillEffects _array_element)))))
    (:then_1
      (Actor|DestroyActor))))

(fn ConstructionScript
  (|CallParentFunction))