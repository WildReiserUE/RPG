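; BP_Skill_MeleeAttack is a short-lived skill actor that delivers a melee hit in front of its owning pawn.
; On BeginPlay, the authority runs a short forward sphere trace for Pawn and WorldDynamic objects, ignoring the owner.
; The hits receive the skill's damage through DamageMultipleEnemies, and each returned target gets the skill effects applied.
; The actor then destroys itself immediately.
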(event EventBeginPlay
  (bind _pawnowner (Variables|Default|GetPawnOwner))
  (bind _returnvalue (Transformation|GetActorLocation _pawnowner))
  (bind _returnvalue_2 (Transformation|GetActorForwardVector _pawnowner))
  (bind _returnvalue_3 (* _returnvalue_2 2e+01))
  (bind _returnvalue_4 (+ _returnvalue _returnvalue_3))
  ;[1 1 1] Deal damage using a sphere trace
  (|CallParentFunction)
  (Utilities|FlowControl|Sequence
    (:then_0
      (Networking|SwitchHasAuthority
        (:Authority
          (bind (_outhits _returnvalue_5) (Collision|MultiSphereTraceForObjects _returnvalue_4 (+ _returnvalue_4 (* (Transformation|GetActorForwardVector (Variables|Default|GetPawnOwner)) 75.0)) 3e+01 (Utilities|Array|MakeArray "ObjectTypeQuery3" "ObjectTypeQuery2") false (Utilities|Array|MakeArray (Variables|Default|GetPawnOwner)) "None"))
          (if _returnvalue_5
            (bind _hitenemies (CallFunction|DamageMultipleEnemies _outhits (Variables|Default|GetSkillDamage) (Variables|Default|GetDamageType)))
            (for _array_element _hitenemies
              (CallFunction|ApplySkillEffects _array_element))))))
    (:then_1
      (Actor|DestroyActor))))

(fn ConstructionScript
  (|CallParentFunction))