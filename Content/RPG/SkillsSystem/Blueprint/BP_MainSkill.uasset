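; BP_MainSkill is the base skill Blueprint, providing shared targeting, damage and effect helpers for RPG skills.
; On BeginPlay it flags AI owners and caches owner and target hostility through interface messages.
; Hostility checks account for duels, AI factions and player-damageable objects, letting multi-hit damage strike each hostile actor only once.
; An authority-gated function passes effects to the target's BP_SkillEffectsComponent, and an interface-based check reports whether targets are alive.
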(event EventBeginPlay
  (bind _skilltarget (Variables|Default|GetSkillTarget))
  ;[1 1 1] See if owner is an aI and set hostility
  (Utilities|FlowControl|Sequence
    (:then_0
      (Utilities|Casting|CastToBP_AI_Main (Variables|Default|GetPawnOwner))
      (Variables|Default|SetOwnerIsAI true))
    (:then_1
      (Utilities|IsValid _skilltarget
        (:Is%20Valid
          (bind _result (Class|ITInteractInterface|GetAIHostility(Message) _skilltarget))
          (Variables|Default|SetTargetHostility _result))))
    (:then_2
      (bind _result_2 (Class|ITInteractInterface|GetAIHostility(Message) (Variables|Default|GetPawnOwner)))
      (Variables|Default|SetOwnerHostility _result_2))))

(fn ConstructionScript)

(fn ApplySkillEffects
  (params (TargetActor :type Actor%20Object%20Reference))
  (bind _applyeffects (Variables|Default|GetApplyEffects))
  (Utilities|IsValid TargetActor
    (:Is%20Valid
      (Utilities|HasAuth
        (:YES
          (if (Utilities|Array|IsValidIndex _applyeffects)
            (bind _output_get (LocalVariables|SetEffectComp (Actor|GetComponentbyClass TargetActor "/Game/RPG/SkillsSystem/Blueprint/SkillComponent/BP_SkillEffectsComponent.BP_SkillEffectsComponent_C")))
            (Utilities|IsValid _output_get
              (:Is%20Valid
                (for _array_element _applyeffects
                  (Default|ApplyEffect _output_get (Variables|Default|GetPawnOwner) _array_element))))))))))

(fn IsTargetHostile
  (params (Target :type Actor%20Object%20Reference))
  (Utilities|FlowControl|Sequence
    (:then_0
      ;[1 1 1] Hostile if dueling
      (bind (_result _dueltarget) (Class|ITSkillEffects|SkillHasDuelTarget(Message) Target))
      (if (and _result (== _dueltarget (Variables|Default|GetPawnOwner)))
        (return true)))
    (:then_1
      (bind _result_2 (Class|ITInteractInterface|GetAIHostility(Message) Target))
      (bind _result_3 (Class|ITInteractInterface|CanbeDamagedbyPlayer?(Message) Target))
      (return (or (and (Math|Boolean|ANDBoolean (Utilities|Enum|Equal(Enum) _result_2 "NewEnumerator3") (not (Variables|Default|GetOwnerIsAI)) _result_3) _result_3) (and (Utilities|Enum|NotEqual(Enum) _result_2 "NewEnumerator3") (Utilities|Enum|NotEqual(Enum) _result_2 (Variables|Default|GetOwnerHostility))))))))

(fn DamageMultipleEnemies
  (params (Array :type Array%20of%20Hit%20Result%20Structures) (BaseDamage :type Float%20%28single-precision%29) (DamageTypeClass :type Damage%20Type%20Class%20Reference))
  ;[1 1 1] Apply damage to enemies, sometimes you might hit multiple bones of the same target and that counts as anotehr hit struct info so we only apply the damage once.
  (for _array_element Array
    (if (and (not (Utilities|Array|ContainsItem (LocalVariables|GetHitTargets) (.HitActor (Collision|BreakHitResult _array_element)))) (CallFunction|IsTargetHostile (.HitActor (Collision|BreakHitResult _array_element))))
      (Utilities|Array|Add (LocalVariables|GetHitTargets) (.HitActor (Collision|BreakHitResult _array_element)))
      (Game|Damage|ApplyDamage (.HitActor (Collision|BreakHitResult _array_element)) BaseDamage 0 (Variables|Default|GetPawnOwner) DamageTypeClass)))
  (return (LocalVariables|GetHitTargets)))

(fn IsTargetAlive?
  (params (TargetRef :type Actor%20Object%20Reference))
  (if (Utilities|DoesObjectImplementInterface TargetRef "/Game/RPG/SkillsSystem/Blueprint/SkillComponent/IT_SkillEffects.IT_SkillEffects_C")
    (bind _result (Class|ITSkillEffects|SkillIsAlive(Message) TargetRef))
    (return _result)
    (else
      (return true))))