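; AC_QuestInfo is a quest data component that serves quest info from a data table for its current quest row.
; GetQuestInfo looks up the current row name through GetQuestInfoByUID, which reuses the cached Info when its unique ID matches and otherwise loads and caches the row.
; SetChainedQuest switches to a different quest row and reloads Info, returning false if the ID is unchanged or the row is missing.
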(fn GetQuestInfo
  (bind _out_row (CallFunction|GetQuestInfobyUID (Variables|Settings|GetQuestRowName)))
  (return _out_row))

(fn SetChainedQuest
  (params (QuestUID :type Name))
  (if (Utilities|Name|NotEqual(Name) QuestUID (Variables|Settings|GetQuestRowName))
    (bind _output_get (Variables|Settings|SetQuestRowName QuestUID))
    (bind _returnvalue (Utilities|GetDataTableRow (Variables|Settings|GetInDataTable) _output_get)
      (:then
        (Variables|Default|SetInfo _returnvalue)
        (return true))
      (:RowNotFound
        _)))
  (return false))

(fn GetQuestInfobyUID
  (params (UID :type Name))
  (Utilities|FlowControl|Sequence
    (:then_0
      (if (Utilities|Name|Equal(Name) (Utilities|Struct|BreakS_QuestInfo (Variables|Default|GetInfo)) UID)
        (return (Variables|Default|GetInfo))))
    (:then_1
      (bind _returnvalue (Utilities|GetDataTableRow (Variables|Settings|GetInDataTable) UID)
        (:then
          (bind _output_get (Variables|Default|SetInfo _returnvalue))
          (return _output_get))
        (:RowNotFound
          (return ""))))))