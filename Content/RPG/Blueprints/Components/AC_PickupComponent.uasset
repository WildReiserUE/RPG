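; Pickup component that holds an item's info struct for an actor, with count, container, equipped state, unique ID, rarity color and mods.
; Initialize fills the struct from a data table row by ItemID; clients also run this lookup on BeginPlay.
; The server rolls random stats once through RandomStatsManager unless stats are passed in.
; Those stats replicate through an OnRep that writes them back into the struct.
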(event Custom|Initialize
  (params (SetStats? :type Boolean) (ItemStats :type Array%20of%20S%20Item%20Stats%20Structures))
  (bind _datasource (Variables|Iteminfo|GetDataSource))
  (bind _output_get (Variables|ItemInfo|SetRandomizeStats? (select SetStats? false (stale _output_get))))
  (Utilities|FlowControl|Sequence
    (:then_0
      (Utilities|IsValid _datasource
        (:Is%20Valid
          (bind _returnvalue (Utilities|GetDataTableRow _datasource (Variables|Iteminfo|GetItem%20ID))
            (:then
              (bind _structout (Utilities|Struct|SetmembersinS_FItemInfo _returnvalue (Utilities|GetClass (Components|GetOwner))))
              (Variables|Default|SetPickupItemInfo _structout)
              (Variables|Default|SetEquipped false)
              (Variables|Default|SetHasUniqueID? false)
              (if (and (Ability|HasAuthority (Components|GetOwner)) (Variables|ItemInfo|GetRandomizeStats?))
                (CallFunction|RandomizeStats)
                (elif (Variables|Default|GetRandomStatsReplicated?)
                  (Utilities|Struct|SetmembersinS_FItemInfo (Variables|Default|GetPickupItemInfo) (Variables|Default|GetRepRandom%20Stats)))))))))
    (:then_1
      (if SetStats?
        (Variables|Default|SetRepRandom%20Stats ItemStats)
        (Variables|Default|SetRandomStatsReplicated? true)
        (Utilities|Struct|SetmembersinS_FItemInfo (Variables|Default|GetPickupItemInfo) (Variables|Default|GetRepRandom%20Stats))))))

(event EventBeginPlay
  (bind _datasource (Variables|Iteminfo|GetDataSource))
  (if (not (Ability|HasAuthority (Components|GetOwner)))
    (Utilities|IsValid _datasource
      (:Is%20Valid
        (bind _returnvalue (Utilities|GetDataTableRow _datasource (Variables|Iteminfo|GetItem%20ID))
          (:then
            (bind _structout (Utilities|Struct|SetmembersinS_FItemInfo _returnvalue (Utilities|GetClass (Components|GetOwner))))
            (Variables|Default|SetPickupItemInfo _structout)
            (Variables|Default|SetEquipped false)
            (Variables|Default|SetHasUniqueID? false)
            (if (and (Ability|HasAuthority (Components|GetOwner)) (Variables|ItemInfo|GetRandomizeStats?))
              (CallFunction|RandomizeStats)
              (elif (Variables|Default|GetRandomStatsReplicated?)
                (Utilities|Struct|SetmembersinS_FItemInfo (Variables|Default|GetPickupItemInfo) (Variables|Default|GetRepRandom%20Stats))))))))))

(fn GetInfo
  (return (Variables|Default|GetPickupItemInfo)))

(fn GetItemNameCount
  (bind _pickupiteminfo (Variables|Default|GetPickupItemInfo))
  (bind (_count _name) (Utilities|Struct|BreakS_FItemInfo _pickupiteminfo))
  (return (Utilities|Text|FormatText "{Name}{Count}" _name (Class|KismetTextLibrary|TexttoLower (select (> _count 1) (Utilities|Text|FormatText " x{count}" (Utilities|Text|ToText(Integer) _count)) (Utilities|Text|MakeLiteralText ""))))))

(fn GetCount
  (return (.Count (Utilities|Struct|BreakS_FItemInfo (Variables|Default|GetPickupItemInfo)))))

(fn UpdateCount
  (params (Count :type Integer))
  (if (> Count 0)
    (Utilities|Struct|SetmembersinS_FItemInfo (Variables|Default|GetPickupItemInfo) Count)
    (return true)
    (else
      (return false))))

(fn SetContainer
  (params (ContainerRef :type BP%20Jig%20Container%20Object%20Reference))
  (Variables|Default|SetContainerRef ContainerRef)
  (return true))

(fn GetContainer
  (return (Variables|Default|GetContainerRef)))

(fn UpdateEquipped
  (params (Equipped :type Boolean))
  (bind _output_get (Variables|Default|SetEquipped Equipped))
  (return _output_get))

(fn SetPickupInfo
  (params (PickupItemInfo :type S%20F%20Item%20Info%20Structure))
  (Variables|Default|SetPickupItemInfo PickupItemInfo)
  (return true))

(fn SetUniqueID
  (params (ID :type Integer))
  (Utilities|Struct|SetmembersinS_FItemInfo (Variables|Default|GetPickupItemInfo) ID)
  (Variables|Default|SetHasUniqueID? true)
  (return true))

(fn HasUniqueID
  (return (Variables|Default|GetHasUniqueID?)))

(fn JustaDummyFunc
  ;[1 1 1] Useless function
  (return (Math|Random|RandomBool)))

(fn GetSpecialContainer
  (return (.SpecialContainerWidget (Utilities|Struct|BreakS_FItemInfo (Variables|Default|GetPickupItemInfo)))))

(fn RandomizeStats
  (bind _pickupiteminfo (Variables|Default|GetPickupItemInfo))
  (bind _randomstats (Utilities|Struct|BreakS_FItemInfo _pickupiteminfo))
  (if (not (Variables|Default|GetStatsRandomized?))
    (Variables|Default|SetStatsRandomized? true)
    (if (> (Utilities|Array|Length (.RollStats (Utilities|Struct|BreakS_JigItemRandomStats _randomstats))) 0)
      (bind _randomstats_2 (Default|GetRandomStats (Variables|Default|GetRandomStatsManager) _randomstats))
      (bind _output_get (Variables|Default|SetRepRandom%20Stats _randomstats_2))
      (Utilities|Struct|SetmembersinS_FItemInfo _pickupiteminfo _output_get))))

(fn OnRepRandomStats
  (Variables|Default|SetRandomStatsReplicated? true)
  (Utilities|Struct|SetmembersinS_FItemInfo (Variables|Default|GetPickupItemInfo) (Variables|Default|GetRepRandom%20Stats)))

(fn GetRarityColor
  (return (Utilities|Select :Index (Utilities|Struct|BreakS_FItemInfo (Variables|Default|GetPickupItemInfo)) :NewEnumerator0 "(R=1.000000,G=1.000000,B=1.000000,A=1.000000)" :NewEnumerator1 "(R=0.000000,G=0.000000,B=1.000000,A=1.000000)" :NewEnumerator2 "(R=1.000000,G=0.000000,B=1.000000,A=1.000000)" :NewEnumerator3 "(R=1.000000,G=0.514956,B=0.000000,A=1.000000)")))

(fn SetCapacity
  (params (Capacity :type Vector%202D%20Structure))
  (Utilities|Struct|SetmembersinS_FItemInfo (Variables|Default|GetPickupItemInfo) Capacity))

(fn GetRarity
  (return (Utilities|Struct|BreakS_FItemInfo (Variables|Default|GetPickupItemInfo))))

(fn SetItemMods
  (params (ItemMods :type Array%20of%20S%20Container%20Items%20Structures))
  (Variables|Default|SetItemMods ItemMods))

(fn GetItemMods
  (return (Variables|Default|GetItemMods)))