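; Actor component that shows its owner's name widget when the cursor hovers over that actor, client-side only.
; On BeginPlay it fetches the local player's inventory component, polls until the controlled pawn is valid, then hands the owner to BP_DisplayName and binds cursor-over events.
; Hover reveals the widget if OutlineOn is set or the pawn is within the inventory component's AI or ground-item distance.
; Cursor exit hides it, and both events broadcast visibility.
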(event Custom|OnBeginCursorOver_Event_0
  (params (TouchedActor :type Actor%20Object%20Reference))
  (bind _pawnref (Variables|Default|GetPawnRef))
  (bind _invcomp (Variables|Default|GetInvComp))
  (if (and (not (Networking|IsDedicatedServer)) (Utilities|IsValid (Variables|Default|GetWidget)))
    (if (and (Pawn|IsLocalController (Game|GetPlayerController 0)) (Utilities|IsValid _pawnref))
      (Variables|Default|SetCurrentVis (Rendering|IsVisible (Variables|Default|GetWidget)))
      (Development|SetHiddeninGame (Variables|Default|GetWidget) (select (Variables|Default|GetOutlineOn) false (not (< (Math|Vector|VectorLength (- (Transformation|GetActorLocation (Components|GetOwner)) (Transformation|GetActorLocation _pawnref))) (Math|Float|SelectFloat (Variables|/Game/RPG/Blueprints/Components/AC_General.AC_General_C|GetAINameVisibiltyDistance _invcomp) (Variables|/Game/RPG/Blueprints/Components/AC_General.AC_General_C|GetNameVisibiltyDistance%28ItemsOnGround%29 _invcomp) (Variables|Default|GetUseAIDistance))))) false)
      (Default|CallOnVisibilityChanged (Rendering|IsVisible (Variables|Default|GetWidget))))))

(event Custom|OnEndCursorOver_Event_0
  (params (TouchedActor :type Actor%20Object%20Reference))
  (Development|SetHiddeninGame (Variables|Default|GetWidget) true false)
  (Default|CallOnVisibilityChanged (Rendering|IsVisible (Variables|Default|GetWidget))))

(event EventBeginPlay
  (bind _returnvalue (Game|GetPlayerController 0))
  (bind _widget (Variables|Default|GetWidget))
  ;[1 1 1] BEGIN PLAY
  (if (not (Networking|IsDedicatedServer))
    (if (Pawn|IsLocalController _returnvalue)
      (bind _inv (Class|BPARPGControllerInterface|GetInventoryComponent(Message) _returnvalue))
      (Variables|Default|SetInvComp _inv)
      (bind _actorref (Class|BPARPGControllerInterface|GetControlledPawnRef(Message) _returnvalue :!label _label))
      (bind _output_get (Variables|Default|SetPawnRef _actorref))
      (Utilities|IsValid _output_get
        (:Is%20Valid
          (Utilities|IsValid _widget
            (:Is%20Valid
              (bind _asbp_display_name (Utilities|Casting|CastToBP_DisplayName (UserInterface|GetUserWidgetObject _widget)))
              (bind _output_get_2 (Variables|/Game/RPG/Widgets/BP_DisplayName.BP_DisplayName_C|SetActorOwner _asbp_display_name (Components|GetOwner)))
              (EventDispatchers|AssignOnBeginCursorOver _output_get_2 (delegate Custom|OnBeginCursorOver_Event_0))
              (EventDispatchers|AssignOnEndCursorOver _output_get_2 (delegate Custom|OnEndCursorOver_Event_0)))))
        (:Is%20Not%20Valid
          (Utilities|FlowControl|Delay 0.2)
          (goto _label)))
      (else
        (Components|Tick|SetComponentTickEnabled false :!label _label_2)))
    (else
      (goto _label_2))))