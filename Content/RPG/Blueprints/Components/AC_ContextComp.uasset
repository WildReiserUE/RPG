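; Context menu component that shows option popups for inventory slots, characters and party members, and also hosts container windows on a lazily created canvas.
; ShowMenu replaces any open menu and remembers its instigator, which OnOptionSelected casts per option.
; Unless the player is stunned, choices route to the inventory component for social server requests or item actions.
; Equip searches for a compatible free container, and Unequip retries with rotated dimensions when space is lacking.
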(fn ShowMenu
  (params (Options :type Array%20of%20E_ContextOptions%20Enums :default "NewEnumerator0") (Caller :type Object%20Object%20Reference))
  (Utilities|FlowControl|Sequence
    (:then_0
      (CallFunction|RemoveMenu))
    (:then_1
      (if (> (Utilities|Array|Length Options) 0)
        (bind _returnvalue (UserInterface|CreateWidget "/Game/RPG/Widgets/ContextMenu/BP_ContextMenuW.BP_ContextMenuW_C" 0 Options self))
        (bind _output_get (Variables|Default|SetMenuRef _returnvalue))
        (Default|Init _output_get)
        (UserInterface|Viewport|AddtoViewport _output_get 4)
        (bind _output_get_2 (Variables|Default|SetMenuInstigator Caller))
        (bind _asbp_jig_slot (Utilities|Casting|CastToBP_JigSlot _output_get_2))
        (Variables|/Game/RPG/Widgets/BP_JigSlot.BP_JigSlot_C|SetCloseMenuOnDestruct _asbp_jig_slot true)))
    (:then_2
      (return))))

(fn RemoveMenu
  (Utilities|FlowControl|Sequence
    (:then_0
      (bind _asbp_jig_slot (Utilities|Casting|CastToBP_JigSlot (Variables|Default|GetMenuInstigator)))
      (Variables|/Game/RPG/Widgets/BP_JigSlot.BP_JigSlot_C|SetCloseMenuOnDestruct _asbp_jig_slot false))
    (:then_1
      (Variables|Default|SetMenuInstigator 0)
      (Utilities|IsValid (Variables|Default|GetMenuRef)
        (:Is%20Valid
          (Widget|RemovefromParent (Variables|Default|GetMenuRef))
          (Variables|Default|SetMenuRef 0)
          (return true))))
    (:then_2
      (return false))))

(fn OnOptionSelected
  (params (Option :type E_ContextOptions%20Enum :default "NewEnumerator0"))
  (bind _returnvalue (Game|GetPlayerController 0))
  (bind _menuinstigator (Variables|Default|GetMenuInstigator))
  (bind _asbp_arpg_character (Utilities|Casting|CastToBP_ARPG_Character _menuinstigator))
  (Variables|Default|SetMenuRef 0)
  (bind _actorref (Class|BPARPGControllerInterface|GetControlledPawnRef(Message) _returnvalue))
  (bind _result (Class|BPISkillEffects|SkillIsStunned?(Message) _actorref))
  (if (not _result)
    (bind _inv (Class|BPARPGControllerInterface|GetInventoryComponent(Message) _returnvalue))
    (bind _output_get (LocalVariables|SetInvComp _inv))
    (switch Utilities|FlowControl|Switch|SwitchonE_ContextOptions Option
      (:NewEnumerator0
        (Default|SERVERRequestPlayerTrade _output_get _asbp_arpg_character))
      (:NewEnumerator1
        (Default|SERVERSendPartyRequest _output_get _asbp_arpg_character))
      (:NewEnumerator2
        (Default|SERVERInvitetoGuild _output_get (.AsActor (Utilities|Casting|CastToActor (Variables|Default|GetMenuInstigator)))))
      (:NewEnumerator3
        (Default|SERVERRequestDUEL _output_get _asbp_arpg_character))
      (:NewEnumerator4
        (bind _asbp_jig_slot (Utilities|Casting|CastToBP_JigSlot (Variables|Default|GetMenuInstigator)))
        (LocalVariables|SetJigItem _asbp_jig_slot)
        (if (and (not (Default|IsEquiptoC (Variables|/Game/RPG/Widgets/BP_JigSlot.BP_JigSlot_C|GetContainerMother _asbp_jig_slot))) (Widget|IsVisible _asbp_jig_slot))
          (bind _returncontainers (Default|GetListOfContainers (Default|GetWidgetInventoryRef (LocalVariables|GetInvComp))))
          (for _array_element _returncontainers
            (if (and (Default|IsEquiptoC _array_element) (not (Default|IsEquipped? _array_element)))
              (if (Default|IsSupportedType? _array_element (Variables|/Game/RPG/Widgets/BP_JigContainer.BP_JigContainer_C|GetSupportedItemTypes _array_element) (.Type (Utilities|Struct|BreakS_FItemInfo (Variables|/Game/RPG/Widgets/BP_JigSlot.BP_JigSlot_C|GetItemInfo _asbp_jig_slot))) (.ItemID (Utilities|Struct|BreakS_FItemInfo (Variables|/Game/RPG/Widgets/BP_JigSlot.BP_JigSlot_C|GetItemInfo _asbp_jig_slot))) (.EquipTo (Utilities|Struct|BreakS_FItemInfo (Variables|/Game/RPG/Widgets/BP_JigSlot.BP_JigSlot_C|GetItemInfo _asbp_jig_slot))) (.SupportedClasses (Utilities|Struct|BreakS_FItemInfo (Variables|/Game/RPG/Widgets/BP_JigSlot.BP_JigSlot_C|GetItemInfo _asbp_jig_slot))))
                (Default|ClientFuncHandleContainertoContainerUnhandled (LocalVariables|GetInvComp) (Variables|/Game/RPG/Widgets/BP_JigSlot.BP_JigSlot_C|GetContainerMother (LocalVariables|GetJigItem)) _array_element (LocalVariables|GetJigItem) 0 0 false)
                (return))))))
      (:NewEnumerator5
        (bind _asbp_jig_slot_2 (Utilities|Casting|CastToBP_JigSlot (Variables|Default|GetMenuInstigator)))
        (LocalVariables|SetJigItem _asbp_jig_slot_2)
        (if (and (Default|IsEquiptoC (Variables|/Game/RPG/Widgets/BP_JigSlot.BP_JigSlot_C|GetContainerMother _asbp_jig_slot_2)) (Widget|IsVisible _asbp_jig_slot_2))
          (bind _output_get_2 (LocalVariables|SetIndex (.SlotIndex (Default|GetEmptySlot (Default|GetMainRef (LocalVariables|GetInvComp)) (.SlotDimension (Utilities|Struct|BreakS_FItemInfo (Variables|/Game/RPG/Widgets/BP_JigSlot.BP_JigSlot_C|GetItemInfo (LocalVariables|GetJigItem))))))))
          (if (!= _output_get_2 -1)
            (Utilities|IsValid (Variables|/Game/RPG/Widgets/BP_JigContainer.BP_JigContainer_C|GetSlotMother (Variables|/Game/RPG/Widgets/BP_JigSlot.BP_JigSlot_C|GetContainerMother (LocalVariables|GetJigItem))) :!label _label
              (:Is%20Valid
                (Default|DropContaineronContainerUnhandledEvent0 (LocalVariables|GetInvComp) (Variables|/Game/RPG/Widgets/BP_JigSlot.BP_JigSlot_C|GetContainerMother (LocalVariables|GetJigItem)) (Default|GetMainRef (LocalVariables|GetInvComp)) (LocalVariables|GetJigItem) 0 (LocalVariables|GetIndex) (LocalVariables|GetRot))
                (return))
              (:Is%20Not%20Valid
                (Default|ClientFuncHandleContainertoContainerUnhandled (LocalVariables|GetInvComp) (Variables|/Game/RPG/Widgets/BP_JigSlot.BP_JigSlot_C|GetContainerMother (LocalVariables|GetJigItem)) (Default|GetMainRef (LocalVariables|GetInvComp)) (LocalVariables|GetJigItem) 0 (LocalVariables|GetIndex) (LocalVariables|GetRot))
                (return)))
            (else
              (LocalVariables|SetIndex (.SlotIndex (Default|GetEmptySlot (Default|GetMainRef (LocalVariables|GetInvComp)) (Math|Vector2D|MakeVector2D (.Y (Math|Vector2D|BreakVector2D (.SlotDimension (Utilities|Struct|BreakS_FItemInfo (Variables|/Game/RPG/Widgets/BP_JigSlot.BP_JigSlot_C|GetItemInfo (LocalVariables|GetJigItem)))))) (.X (Math|Vector2D|BreakVector2D (.SlotDimension (Utilities|Struct|BreakS_FItemInfo (Variables|/Game/RPG/Widgets/BP_JigSlot.BP_JigSlot_C|GetItemInfo (LocalVariables|GetJigItem))))))))))
              (if (!= _output_get_2 -1)
                (LocalVariables|SetRot true)
                (goto _label))))))
      (:NewEnumerator6
        (bind _asbp_jig_slot_3 (Utilities|Casting|CastToBP_JigSlot (Variables|Default|GetMenuInstigator)))
        (bind _returncontainers_2 (Default|GetListOfContainers (Default|GetWidgetInventoryRef (LocalVariables|GetInvComp))))
        (if (Utilities|Array|ContainsItem _returncontainers_2 (Variables|/Game/RPG/Widgets/BP_JigSlot.BP_JigSlot_C|GetContainerMother _asbp_jig_slot_3))
          (Default|ClientFuncHandleDroppingItems (LocalVariables|GetInvComp) _asbp_jig_slot_3 (Default|GetCount _asbp_jig_slot_3) (Variables|/Game/RPG/Widgets/BP_JigSlot.BP_JigSlot_C|GetContainerMother _asbp_jig_slot_3))))
      (:NewEnumerator7
        (bind _asbp_jig_slot_4 (Utilities|Casting|CastToBP_JigSlot (Variables|Default|GetMenuInstigator)))
        (Default|ShowSpecialContainer _asbp_jig_slot_4))
      (:NewEnumerator8
        (bind _asbp_jig_slot_5 (Utilities|Casting|CastToBP_JigSlot (Variables|Default|GetMenuInstigator)))
        (if (or (and (.ReturnValue (Default|IsCapacity? _asbp_jig_slot_5)) (.HasCharges? (Default|IsCapacity? _asbp_jig_slot_5))) (not (.ReturnValue (Default|IsCapacity? _asbp_jig_slot_5))))
          (Default|SERVERRequestConsumeItem _output_get (Default|GetUniqueID _asbp_jig_slot_5) 1)))
      (:NewEnumerator9
        (Default|SERVERLeavePaty (LocalVariables|GetInvComp)))
      (:NewEnumerator10
        (bind _asbp_party_member_w (Utilities|Casting|CastToW_PartyMemberSlot (Variables|Default|GetMenuInstigator)))
        (Default|SERVERPartyKickPlayer (LocalVariables|GetInvComp) (Variables|/Game/RPG/Widgets/W_PartyMemberSlot.W_PartyMemberSlot_C|GetActorOwner _asbp_party_member_w)))
      (:NewEnumerator11
        (bind _asbp_party_member_w_2 (Utilities|Casting|CastToW_PartyMemberSlot (Variables|Default|GetMenuInstigator)))
        (Default|SERVERSetNewLeader (LocalVariables|GetInvComp) (Variables|/Game/RPG/Widgets/W_PartyMemberSlot.W_PartyMemberSlot_C|GetActorOwner _asbp_party_member_w_2))))
    (else
      (Development|PrintString "You can't do that right now!" true true "(R=1.000000,G=0.274510,B=0.000000,A=1.000000)"))))

(fn AddContainerWindow
  (params (WidgetRef :type User%20Widget%20Object%20Reference))
  (Utilities|IsValid (Variables|Default|GetContainerCanvas)
    (:Is%20Valid
      _)
    (:Is%20Not%20Valid
      (bind _returnvalue (UserInterface|CreateWidget "/Game/RPG/Widgets/BP_ContainerCanvas.BP_ContainerCanvas_C"))
      (bind _output_get (Variables|Default|SetContainerCanvas _returnvalue))
      (UserInterface|Viewport|AddtoViewport _output_get 3)))
  (Default|AddNewItem (Variables|Default|GetContainerCanvas) WidgetRef)
  (return))