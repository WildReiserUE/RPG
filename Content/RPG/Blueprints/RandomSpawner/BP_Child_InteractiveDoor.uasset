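; Interactive door, a child in the random spawner family, that toggles open and closed when a character interacts, with optional one-time use.
; Interaction runs on authority or is requested through the component, and notifies the quest component.
; A gated FlipFlop plays or reverses a Timeline that offsets the actor's transform from its construction-time default, reopening the gate on finish.
; Depending on spawner condition, the first completed toggle awards experience and destroys the actor.
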(event Custom|ToggleDoor
  (params (InitiatedBy :type Actor%20Object%20Reference))
  (bind _defaultloc (Variables|Default|GetDefaultLoc))
  (bind _isdooropenbydefault_ (Variables|Settings|GetIsDoorOpenByDefault?))
  (bind _oninteractaddtotransform (Variables|Settings|GetOnInteractAddToTransform))
  (bind _spawnercondition (Variables|Default|GetSpawnerCondition))
  (bind _returnvalue (Utilities|Enum|Equal(Enum) _spawnercondition "NewEnumerator1"))
  ;[0.04167 0.04167 0.04167] Play animation and apply transform
  (Variables|Default|SetActorInteracter InitiatedBy)
  (Utilities|FlowControl|Gate false
    (:Exit
      (bind _isa (Utilities|FlowControl|FlipFlop)
        (:A
          (bind (_direction _loc) (Timeline|Timeline_0 Play)
            (:Update
              (Variables|Default|SetPlayingAnimation? true)
              (Transformation|SetActorTransform (Math|Transform|MakeTransform (+ (.location _defaultloc) (* (.location _oninteractaddtotransform) _loc)) (Math|Rotator|CombineRotators (.rotation _defaultloc) (* (.rotation _oninteractaddtotransform) _loc)) (+ (.scale _defaultloc) (* (.scale _oninteractaddtotransform) _loc))) true))
            (:Finished
              (Variables|Default|SetPlayingAnimation? false)
              (Variables|Default|SetIsDoorOpen (Utilities|Select :Index _direction :Forward (not _isdooropenbydefault_) :Backward _isdooropenbydefault_))
              (CallFunction|OpenGate)
              (if (Variables|Settings|GetHideWidgetNameOnInitialInteraction?)
                (Rendering|SetVisibility (Variables|Default|GetWidget) (not _isa) false))
              (Utilities|FlowControl|DoOnce false
                (:Completed
                  (if (or _returnvalue (Utilities|Enum|Equal(Enum) _spawnercondition "NewEnumerator2"))
                    (if _returnvalue
                      (Class|BPISkillEffects|SkillonTargetExpEarned(Message) (Variables|Default|GetActorInteracter) self (Variables|Default|GetExpEarned) false)
                      (Actor|DestroyActor))))))))
        (:B
          (Timeline|Timeline_0 Reverse))))))

(event Custom|OpenGate
  (bind _defaultloc (Variables|Default|GetDefaultLoc))
  (bind _isdooropenbydefault_ (Variables|Settings|GetIsDoorOpenByDefault?))
  (bind _oninteractaddtotransform (Variables|Settings|GetOnInteractAddToTransform))
  (bind _spawnercondition (Variables|Default|GetSpawnerCondition))
  (bind _returnvalue (Utilities|Enum|Equal(Enum) _spawnercondition "NewEnumerator1"))
  ;[0.04167 0.04167 0.04167] Play animation and apply transform
  (Utilities|FlowControl|Gate false) ; enters at Open
)

(event Custom|ForcedToggle
  (bind _defaultloc (Variables|Default|GetDefaultLoc))
  (bind _isdooropenbydefault_ (Variables|Settings|GetIsDoorOpenByDefault?))
  (bind _oninteractaddtotransform (Variables|Settings|GetOnInteractAddToTransform))
  (bind _spawnercondition (Variables|Default|GetSpawnerCondition))
  (bind _returnvalue (Utilities|Enum|Equal(Enum) _spawnercondition "NewEnumerator1"))
  ;[0.04167 0.04167 0.04167] Play animation and apply transform
  (Utilities|FlowControl|Sequence
    (:then_0
      (goto _label Open))
    (:then_1
      (Utilities|FlowControl|Gate false :!label _label
        (:Exit
          (bind _isa (Utilities|FlowControl|FlipFlop)
            (:A
              (bind (_direction _loc) (Timeline|Timeline_0 Play)
                (:Update
                  (Variables|Default|SetPlayingAnimation? true)
                  (Transformation|SetActorTransform (Math|Transform|MakeTransform (+ (.location _defaultloc) (* (.location _oninteractaddtotransform) _loc)) (Math|Rotator|CombineRotators (.rotation _defaultloc) (* (.rotation _oninteractaddtotransform) _loc)) (+ (.scale _defaultloc) (* (.scale _oninteractaddtotransform) _loc))) true))
                (:Finished
                  (Variables|Default|SetPlayingAnimation? false)
                  (Variables|Default|SetIsDoorOpen (Utilities|Select :Index _direction :Forward (not _isdooropenbydefault_) :Backward _isdooropenbydefault_))
                  (CallFunction|OpenGate)
                  (if (Variables|Settings|GetHideWidgetNameOnInitialInteraction?)
                    (Rendering|SetVisibility (Variables|Default|GetWidget) (not _isa) false))
                  (Utilities|FlowControl|DoOnce false
                    (:Completed
                      (if (or _returnvalue (Utilities|Enum|Equal(Enum) _spawnercondition "NewEnumerator2"))
                        (if _returnvalue
                          (Class|BPISkillEffects|SkillonTargetExpEarned(Message) (Variables|Default|GetActorInteracter) self (Variables|Default|GetExpEarned) false)
                          (Actor|DestroyActor))))))))
            (:B
              (Timeline|Timeline_0 Reverse))))))))

(event EventExecuteInteract
  (params (CharacterRef :type Actor%20Object%20Reference) (Comp :type AC%20General%20Object%20Reference))
  ;[0.04688 0.04688 0.04688] Spawn on interact
  (if (or (not (Variables|Default|GetInteractedOnce)) (not (Variables|Settings|GetOnlyInteractOnce?)))
    (Variables|Default|SetInteractedOnce true)
    (if (Ability|HasAuthority CharacterRef)
      (CallFunction|ToggleDoor CharacterRef)
      (bind _comp (Class|BPQuestInterface|GetQuestComponent(Message) (Components|GetOwner Comp)))
      (Default|QuestTrackonInteractedwith _comp self)
      (else
        (Default|SERVERRequestInteractwithActor Comp self)))))

(fn ConstructionScript
  (|CallParentFunction)
  (Variables|Default|SetDefaultLoc (Transformation|GetActorTransform))
  (Variables|Default|SetIsDoorOpen (Variables|Settings|GetIsDoorOpenByDefault?)))

(fn SetOutlineEnabled
  (params (Enabled :type Boolean) (InteractKey :type Key%20Structure) (CalledFrom :type Actor%20Object%20Reference))
  (bind _outlineon (Variables|Default|GetOutlineOn))
  (|CallParentFunction Enabled InteractKey 0)
  (Rendering|SetRenderCustomDepth (Variables|Default|GetStaticMesh) _outlineon)
  (return _outlineon))

(fn IsDoorOpen?
  (return (Variables|Default|GetIsDoorOpen)))

(fn IsPlayingAnim?
  (return (Variables|Default|GetPlayingAnimation?)))

(fn GetIsDoorOpenPrediction
  (if (CallFunction|IsPlayingAnim?)
    (return (not (Variables|Default|GetIsDoorOpen)))
    (else
      (return (Variables|Default|GetIsDoorOpen)))))

(fn ClearInteraction
  (Variables|Default|SetInteractedOnce false))

(fn GetAcceptableDistance
  (return 2e+02))