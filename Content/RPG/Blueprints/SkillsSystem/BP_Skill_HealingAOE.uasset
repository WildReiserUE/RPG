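; Area-of-effect healing skill that applies its effects to non-hostile pawns around the cursor's world location.
; On BeginPlay, after the parent logic, it runs a multi sphere trace for Pawn objects at that point.
; Non-hostile hit actors are added uniquely to HealedActors, so each receives ApplySkillEffects only once.
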(event EventBeginPlay
  (bind _cursorworldloc (Variables|Default|GetCursorWorldLoc))
  (|CallParentFunction)
  (bind _outhits (Collision|MultiSphereTraceForObjects _cursorworldloc _cursorworldloc 0.0 (Utilities|Array|MakeArray "ObjectTypeQuery3") false 0 "None"))
  (for _array_element _outhits
    (if (not (CallFunction|IsTargetHostile (.HitActor (Collision|BreakHitResult _array_element))))
      (Utilities|Array|AddUnique (Variables|Default|GetHealedActors) (.HitActor (Collision|BreakHitResult _array_element)))))
  (for _array_element_2 (Variables|Default|GetHealedActors)
    (CallFunction|ApplySkillEffects _array_element_2)))

(fn ConstructionScript
  (|CallParentFunction))