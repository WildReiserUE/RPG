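; IT_InteractInterface is a Blueprint interface that defines how the RPG talks to interactable and targetable actors.
; Interaction functions cover executing with a character and component, begin and end hooks, a can-interact check with required duration, and acceptable distance.
; Other functions expose actor name, player damageability, bounty experience, AI behavior, and hostility with color updates for hostile, party or guild status.
; It holds only signatures with default returns, leaving behavior to implementers.
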(fn ExecuteInteract
  (params (CharacterRef :type Actor%20Object%20Reference) (Comp :type BP%20Inventory%20Component%20Object%20Reference)))

(fn CanInteract?
  (return false 0.0))

(fn CanbeDamagedbyPlayer?
  (return false))

(fn GetAcceptableDistance
  (return 0.0))

(fn OnEndInteract
  (return false))

(fn SetHostilityColor
  (params (IsHostile :type Boolean) (IsParty? :type Boolean) (IsGuild? :type Boolean))
  (return false))

(fn GetActorName
  (return ""))

(fn OnBeginInteract
  (return false))

(fn GetAIHostility
  (return "NewEnumerator3"))

(fn SetHostility
  (params (NewHostility :type E_AIHostilityType%20Enum :default "NewEnumerator3"))
  (return false))

(fn GetBountyExp
  (return 0.0))

(fn GetAIBehavior
  (return "NewEnumerator3"))