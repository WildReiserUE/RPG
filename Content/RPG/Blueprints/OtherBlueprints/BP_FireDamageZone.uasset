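; BP_FireDamageZone is a box-trigger hazard that burns and slows actors standing inside it.
; On begin overlap, the server adds an infinite effect with fire damage and a movement slow to the actor's AC_SkillEffects component.
; On end overlap, it removes that effect by its "FireDamageZone" ID, so actors without the component are unaffected and the effect lasts only while inside.
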(event OnComponentBeginOverlap(Box)
  (params (OverlappedComponent :type Primitive%20Component%20Object%20Reference) (OtherActor :type Actor%20Object%20Reference) (OtherComp :type Primitive%20Component%20Object%20Reference) (OtherBodyIndex :type Integer) (bFromSweep :type Boolean) (SweepResult :type Hit%20Result%20Structure%20%28by%20ref%29))
  (Networking|SwitchHasAuthority
    (:Authority
      (bind _output_get (Variables|Default|SetComp (Actor|GetComponentbyClass OtherActor "/Game/RPG/Blueprints/Components/AC_SkillEffects.AC_SkillEffects_C")))
      (Utilities|IsValid _output_get
        (:Is%20Valid
          (Default|AddNewEffect _output_get self (Utilities|Struct|MakeS_SkillEffects "FireDamageZone" "NewEnumerator1" 1e+02 false 0.5 -1.0 1e+01 "/Game/RPG/Blueprints/DamageTypes/BP_FireDamage.BP_FireDamage_C" 0.0 0.0 0.0 0.0 -3e+01)))))))

(event OnComponentEndOverlap(Box)
  (params (OverlappedComponent :type Primitive%20Component%20Object%20Reference) (OtherActor :type Actor%20Object%20Reference) (OtherComp :type Primitive%20Component%20Object%20Reference) (OtherBodyIndex :type Integer))
  (Networking|SwitchHasAuthority
    (:Authority
      (bind _output_get (Variables|Default|SetComp (Actor|GetComponentbyClass OtherActor "/Game/RPG/Blueprints/Components/AC_SkillEffects.AC_SkillEffects_C")))
      (Utilities|IsValid _output_get
        (:Is%20Valid
          (Default|RemoveEffectbyID _output_get "FireDamageZone"))))))

(fn ConstructionScript)