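; RPG game mode that holds back default pawn spawning until a player confirms a character class, then spawns the character at a random PlayerStart.
; The pawn class comes from DT_RaceSetup by race and gender, with a default fallback, and receives the chosen player class.
; A new AI controller possesses the pawn on behalf of the owning PC_Game, which keeps a reference to it.
; On logout, that controlled pawn is destroyed.
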(event Custom|RequestSpawnNewPlayer
  (params (PController :type Player%20Controller%20Object%20Reference))
  ;[1 1 1] Spawn the player when character class is confirmed. (class aka Warrior, Mage etc)
  (CallFunction|SpawnNewPlayer PController (CallFunction|GetRandomSpawnPoint)))

(event EventOnLogout
  (params (ExitingController :type Controller%20Object%20Reference))
  ;[1 1 1] Destroy pawn when player disconnects
  (bind _actorref (Class|BPARPGControllerInterface|GetControlledPawnRef(Message) ExitingController))
  (Utilities|IsValid _actorref
    (:Is%20Valid
      (Actor|DestroyActor _actorref))))

(fn ConstructionScript)

(fn GetRandomSpawnPoint
  ;[1 1 1] Comment
  (bind _outactors (Actor|GetAllActorsOfClass "/Script/Engine.PlayerStart"))
  (return (Math|Transform|MakeTransform (.location (Transformation|GetActorTransform (Utilities|Array|Get(acopy) _outactors (Math|Random|RandomInteger (- (Utilities|Array|Length _outactors) 1))))) (.rotation (Transformation|GetActorTransform (Utilities|Array|Get(acopy) _outactors (Math|Random|RandomInteger (- (Utilities|Array|Length _outactors) 1))))) "1.000000,1.000000,1.000000")))

(fn GetCharacterClassType
  (params (ClassType :type E_ClassTypes%20Enum :default "NewEnumerator0") (RaceType :type E_RaceType%20Enum :default "NewEnumerator6") (GenderType :type E_GenderType%20Enum :default "NewEnumerator2"))
  ;[1 1 1] Return class by race and gender, check out DT_RaceSetup data table to setup your classes to spawn with.
  (bind _outrownames (DataTable|GetDataTableRowNames "/Game/RPG/Blueprints/Character/Lobby/ClassSetups/DT_RaceSetup.DT_RaceSetup"))
  (for _array_element _outrownames
    (bind _returnvalue (Utilities|GetDataTableRow "/Game/RPG/Blueprints/Character/Lobby/ClassSetups/DT_RaceSetup.DT_RaceSetup" _array_element)
      (:then
        (if (Utilities|Enum|Equal(Enum) RaceType (.RaceType (Utilities|Struct|BreakS_RaceSetup _returnvalue)))
          (for _array_element_2 (.CharacterClassByGender (Utilities|Struct|BreakS_RaceSetup _returnvalue))
            (if (Utilities|Enum|Equal(Enum) GenderType (.Gender (Utilities|Struct|BreakS_GenderSetup _array_element_2)))
              (return (.CharacterClass (Utilities|Struct|BreakS_GenderSetup _array_element_2)))))))))
  (Development|PrintString "CLASS TO SPAWN NOT FOUND CHECK DT_RaceSetup config.")
  (return "/Game/RPG/Blueprints/Character/Character_Races/Race1/BP_Character_Race1_Gender1.BP_Character_Race1_Gender1_C"))

(fn SpawnDefaultPawnatTransform
  (params (NewPlayer :type Controller%20Object%20Reference) (SpawnTransform :type Transform%20%28by%20ref%29))
  ;[1 1 1] Override, don't spawn because we are waiting for class confirmation
  (return 0))

(fn SpawnNewPlayer
  (params (PController :type Object%20Object%20Reference) (InputPin :type Transform%20%28by%20ref%29))
  ;[1 1 1] Spawn a new player and assign the correct player controller based on Top down or third person.
  (LocalVariables|SetDefClass (.AsBP%20ARPG%20Character (Utilities|Casting|CastToBP_CharacterClass (Variables|Default|GetDefaultPawnClass))))
  (bind _aspc_game (Utilities|Casting|CastToPC_Game PController))
  (LocalVariables|SetController _aspc_game)
  (bind _returnvalue (Game|SpawnActorfromClass (CallFunction|GetCharacterClassType (Variables|/Game/RPG/Blueprints/Components/AC_General.AC_General_C|GetPlayerClass (Variables|/Game/RPG/Blueprints/PC_Game.PC_Game_C|GetAC_GeneralComponent _aspc_game)) (Variables|/Game/RPG/Blueprints/Components/AC_General.AC_General_C|GetPlayerRace (Variables|/Game/RPG/Blueprints/PC_Game.PC_Game_C|GetAC_GeneralComponent _aspc_game)) (Variables|/Game/RPG/Blueprints/Components/AC_General.AC_General_C|GetPlayerGender (Variables|/Game/RPG/Blueprints/PC_Game.PC_Game_C|GetAC_GeneralComponent _aspc_game))) InputPin "Undefined" 0 (Variables|/Game/RPG/Blueprints/Components/AC_General.AC_General_C|GetPlayerClass (Variables|/Game/RPG/Blueprints/PC_Game.PC_Game_C|GetAC_GeneralComponent _aspc_game)) 0))
  (bind _output_get (LocalVariables|SetPawn _returnvalue))
  (Variables|/Game/RPG/Blueprints/Character/BP_Character.BP_Character_C|SetControllerOwner _output_get (LocalVariables|GetController))
  (bind _returnvalue_2 (Game|SpawnActorfromClass "/Game/RPG/Blueprints/AI/BP_AI_Controller.BP_AI_Controller_C" (Math|Transform|MakeTransform "0, 0, 0") "Undefined" 0 0))
  (Pawn|Possess _returnvalue_2 (LocalVariables|GetPawn))
  (Variables|/Game/RPG/Blueprints/PC_Game.PC_Game_C|SetMyControlledPawn (LocalVariables|GetController) (LocalVariables|GetPawn))
  (Actor|SetOwner _returnvalue_2 (LocalVariables|GetController))
  ;;[0.07292 0.07292 0.07292] Must return nothing to handle possessing ourselves
  (return 0))

(fn GetDefaultPawnClassforController
  (params (InController :type Controller%20Object%20Reference))
  (bind _returnvalue (|CallParentFunction InController))
  (return _returnvalue))