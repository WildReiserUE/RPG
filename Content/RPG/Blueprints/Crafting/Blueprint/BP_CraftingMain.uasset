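; Interactable crafting NPC that shows its name overhead, cannot be damaged by players, and opens a crafting window.
; On interaction it passes itself to the interactor's component, while its CraftingWidgetComponent shows, closes and reports on the window.
; Modular gear meshes follow the body through master pose.
; Highlighting uses custom depth on the body and most gear, and updates the interact key on the name widget.
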(event EventBeginPlay
  (bind _widget (Variables|Default|GetWidget))
  (bind _returnvalue (UserInterface|GetUserWidgetObject _widget))
  ;[1 1 1] Set character name on the WidgetComponent
  (Utilities|IsValid _returnvalue
    (:Is%20Valid
      (bind _asbp_display_name (Utilities|Casting|CastToBP_DisplayName _returnvalue))
      (Default|UpdateName _asbp_display_name (Variables|Settings|GetCharacterName) "(R=1.000000,G=1.000000,B=1.000000,A=1.000000)"))))

(event EventExecuteInteract
  (params (CharacterRef :type Actor%20Object%20Reference) (Comp :type AC%20General%20Object%20Reference))
  ;[1 1 1] When interacted with
  (Default|ShowCraftWidget Comp self))

(fn ConstructionScript
  (Class|SkinnedMeshComponent|SetMasterPoseComponent (Variables|Default|GetArmor) (Variables|Character|GetMesh) false)
  (Variables|/Game/RPG/Blueprints/Components/AC_NameVisibility.AC_NameVisibility_C|SetWidget (Variables|Default|GetBP_NameVisibility) (Variables|Default|GetWidget)))

(fn ShowContent
  (params (InvComp :type AC%20General%20Object%20Reference))
  ;[1 1 1] Show crafting widget
  (Default|ShowWidget (Variables|Default|GetCraftingWidgetComponent) (Variables|Settings|GetCharacterName) InvComp (Variables|Settings|GetRollRandomStats?)))

(fn CloseWidget
  ;[1 1 1] Close crafting widget
  (Widget|RemovefromParent (Variables|/Game/RPG/Blueprints/Components/AC_CraftingWidget.AC_CraftingWidget_C|GetWidgetRef (Variables|Default|GetCraftingWidgetComponent))))

(fn GetWidgetRef
  ;[1 1 1] Get crafing widget reference
  (return (Variables|/Game/RPG/Blueprints/Components/AC_CraftingWidget.AC_CraftingWidget_C|GetWidgetRef (Variables|Default|GetCraftingWidgetComponent))))

(fn IsWVisible
  (bind _craftingwidgetcomponent (Variables|Default|GetCraftingWidgetComponent))
  (bind _widgetref (Variables|/Game/RPG/Blueprints/Components/AC_CraftingWidget.AC_CraftingWidget_C|GetWidgetRef _craftingwidgetcomponent))
  ;[1 1 1] Checks if crafting widget is visibe
  (Utilities|IsValid _widgetref
    (:Is%20Valid
      (return (Widget|IsVisible _widgetref)))
    (:Is%20Not%20Valid
      (return false))))

(fn CanbeDamagedbyPlayer?
  (return false))

(fn CanInteract?
  (return true 0.0))

(fn GetAcceptableDistance
  (return 1e+02))

(fn GetActorName
  (return ""))

(fn GetAIBehavior
  (return "NewEnumerator3"))

(fn GetAIHostility
  (return "NewEnumerator3"))

(fn GetBountyExp
  (return 0.0))

(fn GetOutlineColor
  (return "(R=0.000000,G=0.824136,B=1.000000,A=1.000000)"))

(fn OnBeginInteract
  (return false))

(fn OnEndInteract
  (return false))

(fn SetHostility
  (params (NewHostility :type E_AIHostilityType%20Enum :default "NewEnumerator3"))
  (return false))

(fn SetHostilityColor
  (params (IsHostile :type Boolean) (IsParty? :type Boolean) (IsGuild? :type Boolean))
  (return false))

(fn SetOutlineEnabled
  (params (Enabled :type Boolean) (InteractKey :type Key%20Structure) (CalledFrom :type Actor%20Object%20Reference))
  (bind _nonekey (LocalVariables|GetNoneKey))
  (bind _returnvalue (== InteractKey _nonekey))
  ;[1 1 1] Set outline, the key value is used in third person mode
  (bind _output_get (Variables|/Game/RPG/Blueprints/Components/AC_NameVisibility.AC_NameVisibility_C|SetOutlineOn (Variables|Default|GetBP_NameVisibility) Enabled))
  (Rendering|SetRenderCustomDepth (Variables|Character|GetMesh) _output_get)
  (Utilities|FlowControl|Sequence
    (:then_0
      (if (not _returnvalue)
        (bind _asbp_display_name (Utilities|Casting|CastToBP_DisplayName (UserInterface|GetUserWidgetObject (Variables|Default|GetWidget))))
        (Default|SetInteractKey _asbp_display_name (Class|KismetInputLibrary|KeyGetDisplayName InteractKey) (or _returnvalue (not _output_get)))))
    (:then_1
      (return Enabled))))