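; Lobby character preview actor that shows a race and gender body with equipped gear, built from either class settings or an item list.
; Race and gender select mesh and looping pose from DT_PreviewLobbyCharSettings.
; SpawnAndEquip resolves item data-table rows to class/race/gender-filtered equipment actors, attaching them to main or off-hand sockets.
; Worn pieces follow the body through master pose, and spawned gear stays hidden until attached to avoid visible snapping.
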(fn ConstructionScript)

(fn SetCharacterHidden
  (params (bNewHidden :type Boolean))
  (Rendering|SetActorHiddenInGame bNewHidden)
  (for _array_element (Variables|Default|GetSpawnedActors)
    (Rendering|SetActorHiddenInGame _array_element bNewHidden)))

(fn SetEquipmentbyClass
  (params (ClasSettings :type S%20Class%20Setups%20Structure%20%28by%20ref%29) (PClass :type E_ClassTypes%20Enum :default "NewEnumerator0") (PRace :type E_RaceType%20Enum :default "NewEnumerator6") (PGender :type E_GenderType%20Enum :default "NewEnumerator2"))
  (bind (_equippedprimary _equippedsecondary _equippedarmor _equippedpants _equippedboots) (Utilities|Struct|BreakS_ClassSetups ClasSettings))
  (bind _spawnedactors (Variables|Default|GetSpawnedActors))
  (bind (_itemid _indatatable) (Utilities|Struct|BreakS_StartingItems _equippedsecondary))
  (bind (_itemid_2 _indatatable_2) (Utilities|Struct|BreakS_StartingItems _equippedprimary))
  (bind (_itemid_3 _indatatable_3) (Utilities|Struct|BreakS_StartingItems _equippedarmor))
  (bind (_itemid_4 _indatatable_4) (Utilities|Struct|BreakS_StartingItems _equippedpants))
  (bind (_itemid_5 _indatatable_5) (Utilities|Struct|BreakS_StartingItems _equippedboots))
  (Utilities|FlowControl|Sequence
    (:then_0
      (for _array_element _spawnedactors
        (Actor|DestroyActor _array_element))
      (Utilities|Array|Clear _spawnedactors))
    (:then_1
      (CallFunction|SpawnandEquip _indatatable_2 _itemid_2 false PClass PRace PGender false)
      (CallFunction|SpawnandEquip _indatatable _itemid true PClass PRace PGender false)
      (CallFunction|SpawnandEquip _indatatable_3 _itemid_3 false PClass PRace PGender true)
      (CallFunction|SpawnandEquip _indatatable_4 _itemid_4 false PClass PRace PGender true)
      (CallFunction|SpawnandEquip _indatatable_5 _itemid_5 false PClass PRace PGender true)
      ;[1 1 1] Removes attach snapping visual issue.
      (for _array_element_2 (Variables|Default|GetSpawnedActors)
        (Rendering|SetActorHiddenInGame _array_element_2 false)))))

(fn SpawnandEquip
  (params (DataTable :type Data%20Table%20Object%20Reference) (RowName :type Name) (OffHand? :type Boolean) (PClass :type E_ClassTypes%20Enum :default "NewEnumerator0") (PRace :type E_RaceType%20Enum :default "NewEnumerator6") (PGender :type E_GenderType%20Enum :default "NewEnumerator2") (SetMasterPose? :type Boolean))
  (Utilities|FlowControl|Sequence
    (:then_0
      (if (and (Utilities|IsValid DataTable) (Utilities|Name|NotEqual(Name) RowName "None"))
        (bind _returnvalue (Utilities|GetDataTableRow DataTable RowName)
          (:then
            (bind _output_get (LocalVariables|SetClassToUse (CallFunction|GetEquipmentClass _returnvalue PClass PRace PGender)))
            (if (Utilities|IsValidClass _output_get)
              (bind _returnvalue_2 (Game|SpawnActorfromClass _output_get (Math|Transform|MakeTransform "0, 0, 0" "0, 0, 0" "1,1,1") "AlwaysSpawn" 0 0))
              (Utilities|Array|Add (Variables|Default|GetSpawnedActors) _returnvalue_2)
              (Transformation|AttachComponentToComponent _returnvalue_2 (CallFunction|GetSkeletalMeshReference) (select OffHand? (.EquipToOffHandSocket (Utilities|Struct|BreakS_FItemInfo _returnvalue)) (.EquipToMainHandSocket (Utilities|Struct|BreakS_FItemInfo _returnvalue))) "SnapToTarget" "SnapToTarget" "KeepWorld" true)
              (Rendering|SetActorHiddenInGame _returnvalue_2 true)
              (Utilities|FlowControl|Sequence
                (:then_0
                  (if SetMasterPose?
                    (Class|SkinnedMeshComponent|SetMasterPoseComponent (Variables|/Game/RPG/Blueprints/Equipment/BP_MainEquipment.BP_MainEquipment_C|GetMainSkelMesh _returnvalue_2) (CallFunction|GetSkeletalMeshReference) false)))
                (:then_1
                  (return _returnvalue_2 (select OffHand? (.EquipToOffHandSocket (Utilities|Struct|BreakS_FItemInfo _returnvalue)) (.EquipToMainHandSocket (Utilities|Struct|BreakS_FItemInfo _returnvalue)))))))))))
    (:then_1
      (return 0 "None"))))

(fn SetMainEquipment
  (params (Items :type Array%20of%20S%20Starting%20Items%20Structures) (Race :type E_RaceType%20Enum :default "NewEnumerator6") (Gender :type E_GenderType%20Enum :default "NewEnumerator2"))
  (bind _spawnedactors (Variables|Default|GetSpawnedActors))
  (CallFunction|SetRaceandGender Race Gender)
  (Utilities|FlowControl|Sequence
    (:then_0
      (for _array_element _spawnedactors
        (Actor|DestroyActor _array_element))
      (Utilities|Array|Clear _spawnedactors))
    (:then_1
      (for (_array_element_2 _array_index) Items
        (bind (_returnvalue _attackedto) (CallFunction|SpawnandEquip (.InDataTable (Utilities|Struct|BreakS_StartingItems _array_element_2)) (.ItemID (Utilities|Struct|BreakS_StartingItems _array_element_2)) (or (== (.Count (Utilities|Struct|BreakS_StartingItems _array_element_2)) -7) (== _array_index 14)) "NewEnumerator0" "NewEnumerator6" "NewEnumerator2" false))
        (Utilities|IsValid _returnvalue
          (:Is%20Valid
            (if (Utilities|Name|Equal(Name) _attackedto "None")
              (Rendering|SetActorHiddenInGame _returnvalue true)
              (Class|SkinnedMeshComponent|SetMasterPoseComponent (Variables|/Game/RPG/Blueprints/Equipment/BP_MainEquipment.BP_MainEquipment_C|GetMainSkelMesh _returnvalue) (CallFunction|GetSkeletalMeshReference) false)))))
      (for _array_element_3 (Variables|Default|GetSpawnedActors)
        (Rendering|SetActorHiddenInGame _array_element_3 false)))))

(fn GetEquipmentClass
  (params (Info :type S%20F%20Item%20Info%20Structure%20%28by%20ref%29) (PClass :type E_ClassTypes%20Enum%20%28by%20ref%29 :default "NewEnumerator0") (PRace :type E_RaceType%20Enum%20%28by%20ref%29 :default "NewEnumerator6") (PGender :type E_GenderType%20Enum%20%28by%20ref%29 :default "NewEnumerator2"))
  (bind (_equipmenttoequip _equipmentsetup) (Utilities|Struct|BreakS_FItemInfo Info))
  (Utilities|FlowControl|Sequence
    (:then_0
      (for _array_element _equipmentsetup
        (if (Math|Boolean|ANDBoolean (Math|Boolean|ORBoolean (Utilities|Array|ContainsItem (.SupportedClasses (Utilities|Struct|BreakS_EquipmentSetup _array_element)) PClass) (Utilities|Array|ContainsItem (.SupportedClasses (Utilities|Struct|BreakS_EquipmentSetup _array_element)) "NewEnumerator0") (== (Utilities|Array|Length (.SupportedClasses (Utilities|Struct|BreakS_EquipmentSetup _array_element))) 0)) (Math|Boolean|ORBoolean (Utilities|Array|ContainsItem (.SupportedRaces (Utilities|Struct|BreakS_EquipmentSetup _array_element)) PRace) (Utilities|Array|ContainsItem (.SupportedRaces (Utilities|Struct|BreakS_EquipmentSetup _array_element)) "NewEnumerator6") (== (Utilities|Array|Length (.SupportedRaces (Utilities|Struct|BreakS_EquipmentSetup _array_element))) 0)) (Math|Boolean|ORBoolean (Utilities|Array|ContainsItem (.SupportedGenders (Utilities|Struct|BreakS_EquipmentSetup _array_element)) PGender) (Utilities|Array|ContainsItem (.SupportedGenders (Utilities|Struct|BreakS_EquipmentSetup _array_element)) "NewEnumerator2") (== (Utilities|Array|Length (.SupportedGenders (Utilities|Struct|BreakS_EquipmentSetup _array_element))) 0)))
          (return (.EquipmentClass (Utilities|Struct|BreakS_EquipmentSetup _array_element))))))
    (:then_1
      (return _equipmenttoequip))))

(fn SetRaceandGender
  (params (Race :type E_RaceType%20Enum :default "NewEnumerator6") (Gender :type E_GenderType%20Enum :default "NewEnumerator2"))
  (bind _skelref (CallFunction|GetSkeletalMeshReference))
  ;[1 1 1] Use info from data table to set the mesh and animation
  (bind _outrownames (DataTable|GetDataTableRowNames "/Game/RPG/Blueprints/Character/Lobby/ClassSetups/DT_PreviewLobbyCharSettings.DT_PreviewLobbyCharSettings"))
  (for _array_element _outrownames
    (bind _returnvalue (Utilities|GetDataTableRow "/Game/RPG/Blueprints/Character/Lobby/ClassSetups/DT_PreviewLobbyCharSettings.DT_PreviewLobbyCharSettings" _array_element)
      (:then
        (if (Utilities|Enum|Equal(Enum) (.RaceType (Utilities|Struct|BreakS_LobbyCharPreviewSetup _returnvalue)) Race)
          (for _array_element_2 (.MeshByGender (Utilities|Struct|BreakS_LobbyCharPreviewSetup _returnvalue))
            (if (Utilities|Enum|Equal(Enum) (.GenderType (Utilities|Struct|BreakS_LobbyCharPreviewMeshByGender _array_element_2)) Gender)
              (Utilities|FlowControl|Sequence
                (:then_0
                  (if (!= (Variables|/Script/Engine.SkinnedMeshComponent|GetSkeletalMesh (CallFunction|GetSkeletalMeshReference)) (.Mesh (Utilities|Struct|BreakS_LobbyCharPreviewMeshByGender _array_element_2)))
                    (Class|SkinnedMeshComponent|SetSkeletalMesh _skelref (.Mesh (Utilities|Struct|BreakS_LobbyCharPreviewMeshByGender _array_element_2)) true))
                  (if (!= (Utilities|Struct|BreakSingleAnimationPlayData (Variables|/Script/Engine.SkeletalMeshComponent|GetAnimationData (CallFunction|GetSkeletalMeshReference))) (.PoseAnimation (Utilities|Struct|BreakS_LobbyCharPreviewMeshByGender _array_element_2)))
                    (Components|Animation|PlayAnimation _skelref (.PoseAnimation (Utilities|Struct|BreakS_LobbyCharPreviewMeshByGender _array_element_2)) true)))
                (:then_1
                  (return))))))))))

(fn ClearCharacter
  (bind _spawnedactors (Variables|Default|GetSpawnedActors))
  (for _array_element _spawnedactors
    (Actor|DestroyActor _array_element))
  (Utilities|Array|Clear _spawnedactors)
  (Class|SkinnedMeshComponent|SetSkeletalMesh (CallFunction|GetSkeletalMeshReference) 0 false))

(fn GetSkeletalMeshReference
  (return (Variables|Default|GetSkeletalMesh)))