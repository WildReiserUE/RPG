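; Behavior tree task that points the AI at the last known location of its enemy.
; On execute it clears the UseLastKnowLoc flag, copies LastEnemyKnowLoc into the TargetLocation blackboard key and finishes successfully, without issuing the move itself.
; An unconnected optional branch would raise the BP_AI_Main pawn's walk speed to its sprint speed so it runs there instead of walking.
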(event EventReceiveExecuteAI
  (params (OwnerController :type AI%20Controller%20Object%20Reference) (ControlledPawn :type Pawn%20Object%20Reference))
  (Utilities|FlowControl|Sequence
    (:then_1
      (Class|BTFunctionLibrary|SetBlackboardValueasBool (Variables|Default|GetUseLastKnowLoc) false)
      (AI|BehaviorTree|SetBlackboardValueasVector (Variables|Default|GetTargetLocation) (Class|BTFunctionLibrary|GetBlackboardValueasVector (Variables|Default|GetLastEnemyKnowLoc)))
      (AI|BehaviorTree|FinishExecute true))))