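; Behavior tree task that picks the next TargetLocation for a BP_AI_Main pawn.
; Stationary AI receive their stationary location and always finish successfully.
; Other AI receive a random navigable point within the HomeRaduis around HomeLocation from the blackboard, and the task succeeds only if that lookup succeeds.
; A failed cast to BP_AI_Main never calls FinishExecute.
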(event EventReceiveExecuteAI
  (params (OwnerController :type AI%20Controller%20Object%20Reference) (ControlledPawn :type Pawn%20Object%20Reference))
  (bind _asbp_ai_main (Utilities|Casting|CastToBP_AI_Main ControlledPawn))
  (if (.IsStationaryAI (Default|IsStationary _asbp_ai_main))
    (AI|BehaviorTree|SetBlackboardValueasVector (Variables|Default|GetTargetLocation) (.Location (Math|Transform|BreakTransform (.StationaryLocation (Default|IsStationary _asbp_ai_main)))))
    (AI|BehaviorTree|FinishExecute true)
    (else
      (bind (_randomlocation _returnvalue) (Class|NavigationSystemV1|GetRandomLocationinNavigableRadius (Class|BTFunctionLibrary|GetBlackboardValueasVector (Variables|Default|GetHomeLocation)) (Class|BTFunctionLibrary|GetBlackboardValueasFloat (Variables|Default|GetHomeRaduis)) 0 0))
      (AI|BehaviorTree|SetBlackboardValueasVector (Variables|Default|GetTargetLocation) _randomlocation)
      (AI|BehaviorTree|FinishExecute _returnvalue))))