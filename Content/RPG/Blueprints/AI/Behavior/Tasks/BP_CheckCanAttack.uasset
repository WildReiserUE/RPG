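; Behavior tree task that checks whether a BP_AI_Main pawn can attack and prepares its next attack.
; It clears controller focus, then fails if the pawn is attacking or stunned.
; Otherwise it selects the next attack, writes that attack's range to the AttackRange blackboard key, and sets a new target, succeeding only if the target is valid.
; A failed pawn cast stops execution without finishing the task.
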(event EventReceiveExecuteAI
  (params (OwnerController :type AI%20Controller%20Object%20Reference) (ControlledPawn :type Pawn%20Object%20Reference))
  (AI|ClearFocus OwnerController)
  (bind _asbp_ai_main (Utilities|Casting|CastToBP_AI_Main ControlledPawn))
  (if (or (Default|IsAttacking? _asbp_ai_main) (Default|IsStunned? _asbp_ai_main))
    (AI|BehaviorTree|FinishExecute false)
    (else
      (bind _attackrange (Default|SelectNextAttack _asbp_ai_main))
      (Class|BTFunctionLibrary|SetBlackboardValueasFloat (Variables|Default|GetAttackRange) _attackrange)
      (bind _output_get (Default|SetNewTarget _asbp_ai_main))
      (AI|BehaviorTree|FinishExecute (Utilities|IsValid _output_get)))))