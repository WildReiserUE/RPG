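; Behavior tree task that moves an AI character to the friendly actor stored in the Blackboard.
; On execute it calls AI MoveTo with a tight acceptance radius for a moving friendly and a randomized one for a stationary one, succeeding immediately if stunned.
; Each tick it selects sprint speed when the friendly is both nearby and moving quickly, otherwise normal speed, and fails if the friendly becomes invalid.
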(event EventReceiveExecuteAI
  (params (OwnerController :type AI%20Controller%20Object%20Reference) (ControlledPawn :type Pawn%20Object%20Reference))
  (bind _output_get (Variables|Default|SetFriendlyRef (AI|BehaviorTree|GetBlackboardValueasActor (Variables|Default|GetFriendly))))
  (Utilities|IsValid _output_get
    (:Is%20Valid
      (bind _asbp_ai_main (Utilities|Casting|CastToBP_AI_Character ControlledPawn))
      (bind _output_get_2 (Variables|Default|SetOwnerChar _asbp_ai_main))
      (if (Default|IsStunned? _output_get_2)
        (AI|BehaviorTree|FinishExecute true)
        (else
          (AI|AIMoveTo OwnerController "0, 0, 0" (Variables|Default|GetFriendlyRef) (Math|Random|RandomFloatinRange 1e+02 (Math|Float|SelectFloat 1e+02 5e+02 (> (Math|Vector|VectorLength (Transformation|GetVelocity (Variables|Default|GetFriendlyRef))) 0.0))) "Default" "Default" true false
            (:OnRequestFailed
              (AI|BehaviorTree|FinishExecute false))
            (:OnMoveFinished
              (AI|BehaviorTree|FinishExecute true))))))
    (:Is%20Not%20Valid
      (AI|BehaviorTree|FinishExecute false))))

(event EventReceiveTickAI
  (params (OwnerController :type AI%20Controller%20Object%20Reference) (ControlledPawn :type Pawn%20Object%20Reference) (DeltaSeconds :type Float%20%28single-precision%29))
  (bind _ownerchar (Variables|Default|GetOwnerChar))
  (bind _friendlyref (Variables|Default|GetFriendlyRef))
  (bind _aistats (Variables|/Game/RPG/Blueprints/AI/BP_AI_Character.BP_AI_Character_C|GetAIStats _ownerchar))
  (bind (_movementspeed _sprintspeed) (Utilities|Struct|BreakS_AIStats _aistats))
  (Utilities|IsValid (Variables|Default|GetFriendlyRef)
    (:Is%20Valid
      (Variables|/Script/Engine.CharacterMovementComponent|SetMaxWalkSpeed (Variables|/Script/Engine.Character|GetCharacterMovement (Variables|Default|GetOwnerChar)) (Math|Float|SelectFloat _movementspeed _sprintspeed (or (> (Math|Vector|VectorLength (- (Transformation|GetActorLocation ControlledPawn) (Transformation|GetActorLocation _friendlyref))) 1e+03) (< (Math|Vector|VectorLength (Transformation|GetVelocity _friendlyref)) 2e+02)))))
    (:Is%20Not%20Valid
      (AI|BehaviorTree|FinishExecute false))))